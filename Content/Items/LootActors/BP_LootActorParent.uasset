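; Parent actor for lootable chests and dropped loot bags, with loot held in a LootComponent and an outline setup.
; Interact runs on authority, locks the container to one character and flips replicated Open, whose OnRep triggers animation and movement locking.
; OC_Inventory toggles the local loot menu.
; A timer polls for the player's QuestReceiverComponent, then binds a handler that sends this actor's location for matching tracked loot objectives.
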(event Custom|OC_Inventory
  (params (CharacterRef :type Character%20Object%20Reference))
  ;[1 1 1] Interact - Open Loot
  ;;[1 1 1] Toggle Chest Widget
  (Variables|Default|SetCharacterRef CharacterRef)
  ;;;[1 1 1] Open Loot Menu & Save Data
  (Class|IPlayerController|ToggleLootMenu(Message) (Game|GetPlayerController 0) (Variables|Default|GetLootComponent))
  (if (Variables|Default|GetOpen)
    (Default|SetFocus (Variables|Default|GetLootComponent))
    (else
      (Pawn|Components|CharacterMovement|SetMovementMode (Variables|/Script/Engine.Character|GetCharacterMovement (Variables|Default|GetCharacterRef)) "MOVE_Walking" 0))))

(event Custom|PlayerValidCheck
  ;[1 1 1] Binds Dispatcher To Pass Location if Kill Quest Objective
  (Utilities|IsValid (Actor|GetComponentbyClass (Game|GetPlayerCharacter 0) "/Game/FlexibleCombatSystem/Blueprints/Components/QuestReceiverComponent.QuestReceiverComponent_C")
    (:Is%20Valid
      (Utilities|Time|ClearandInvalidateTimerbyHandle (stale EventBeginPlay _returnvalue))
      (EventDispatchers|BindEventtoQuestObjectiveLink (Actor|GetComponentbyClass (Game|GetPlayerCharacter 0) "/Game/FlexibleCombatSystem/Blueprints/Components/QuestReceiverComponent.QuestReceiverComponent_C") (EventDispatchers|CreateEvent :!event BPLootActorParentAutoGenFunc)))))

(event EventBeginPlay
  ;[1 1 1] Binds Dispatcher To Pass Location if Kill Quest Objective
  (bind _returnvalue (Utilities|Time|SetTimerbyEvent (delegate Custom|PlayerValidCheck) 2.0 true)))

(event EventAddLoottoDroppedLoot
  (params (DroppedItem :type S%20Slot%20Info%20Structure))
  ;[1 1 1] Interact - Open Loot
  (Default|AddLootDataRemake (Variables|Default|GetLootComponent) DroppedItem))

(event EventToggleNotifyforAnim
  ;[1 1 1] Interact - Open Loot
  (Variables|Default|SetOpen (not (Variables|Default|GetOpen))))

(event EventInteract
  (params (Character :type Character%20Object%20Reference))
  ;[1 1 1] Interact - Open Loot
  ;;[1 1 1] Run On Server
  (if (Variables|Default|GetOpen)
    (if (== (Variables|Default|GetCharacterRef) Character)
      (if (not (Variables|/Game/FlexibleCombatSystem/Blueprints/Components/LootComponent.LootComponent_C|GetActorLooted (Variables|Default|GetLootComponent))) :!label _label
        (Networking|SwitchHasAuthority
          (:Authority
            (bind _output_get (Variables|Default|SetCharacterRef Character))
            (Actor|SetOwner _output_get)
            ;;;[1 1 1] Handles Opening the Chest Via Notify
            (Variables|Default|SetOpen (not (Variables|Default|GetOpen)))
            (CallFunction|OCInventory (Variables|Default|GetCharacterRef)))))
      (elif (Pawn|IsLocallyControlled Character)
        (bind _returnvalue (UserInterface|CreateWidget "/Game/FlexibleCombatSystem/Widgets/Combat/WB_PopupText.WB_PopupText_C" 0 "Loot in Use!"))
        (UserInterface|Viewport|AddtoViewport _returnvalue 0)))
    (else
      (goto _label))))

(fn ConstructionScript)

(fn BPLootActorParentAutoGenFunc
  (params (Quest%20Receiver :type Quest%20Receiver%20Component%20Object%20Reference) (Quest%20Info :type S%20Quest%20Info%20Structure))
  ;[1 1 1] IF Quest Item is Part of Quest Pass Data (Updated Location) over to Quest Log
  (bind (_array_element _array_index) (Utilities|Array|ForEachLoopwithBreak (Utilities|Struct|BreakS_QuestInfo Quest%20Info) :!label _label)
    (:LoopBody
      (if (.ObjectiveHasTracking? (Utilities|Struct|BreakS_QuestObjectiveInfo _array_element))
        (bind _returnvalue (Game|GetCurrentLevelName true))
        (if (Utilities|Enum|Equal(Enum) _returnvalue (.ObjectiveMapName (Utilities|Struct|BreakS_QuestObjectiveInfo _array_element)))
          (if (Utilities|Enum|Equal(Enum) (.LootName (Utilities|Struct|BreakS_LootSetupInfo (Variables|SetupinGame|GetLootSetupInfo))) (.ContainerNameIFItemLootedfromEnemyorChest (Utilities|Struct|BreakS_QuestObjectiveInfo _array_element)))
            (bind _array_element_2 (Utilities|Array|ForEachLoopwithBreak (.PiecesOfLoot (Utilities|Struct|BreakS_LootSetupInfo (Variables|SetupinGame|GetLootSetupInfo))))
              (:LoopBody
                (if (Utilities|Enum|Equal(Enum) (Utilities|Struct|BreakS_ItemData (CallFunction|GetItemData (Utilities|Struct|BreakS_ItemSetupData _array_element_2))) (.ObjectiveName (Utilities|Struct|BreakS_QuestObjectiveInfo _array_element)))
                  (Default|PassObjectiveUpdatedLocation Quest%20Receiver (Utilities|Struct|MakeS_QuestObjectiveInfo (.ObjectiveName (Utilities|Struct|BreakS_QuestObjectiveInfo _array_element)) (.ContainerNameIFItemLootedfromEnemyorChest (Utilities|Struct|BreakS_QuestObjectiveInfo _array_element)) (.ObjectiveType (Utilities|Struct|BreakS_QuestObjectiveInfo _array_element)) (.TotalObjectiveNumber (Utilities|Struct|BreakS_QuestObjectiveInfo _array_element)) (.ObjectiveHasTracking? (Utilities|Struct|BreakS_QuestObjectiveInfo _array_element)) (.ObjectiveMapName (Utilities|Struct|BreakS_QuestObjectiveInfo _array_element)) (Transformation|GetActorLocation) self) _array_index)
                  (goto _label Break))))))))))

(fn OnRepOpen
  (Class|ILootInterface|ToggleAnimation(Message) self)
  (bind _gamepad (Class|IPlayerController|PassControlInput(Message) (Game|GetPlayerController 0)))
  (if _gamepad
    (if (Variables|Default|GetOpen)
      (Pawn|Components|CharacterMovement|DisableMovement (Variables|/Script/Engine.Character|GetCharacterMovement (Variables|Default|GetCharacterRef)))
      (else
        (Pawn|Components|CharacterMovement|SetMovementMode (Variables|/Script/Engine.Character|GetCharacterMovement (Variables|Default|GetCharacterRef)) "MOVE_Walking" 0)))))

(fn InitializeDroppedLoot
  (Default|SetupOutlineVariables (Variables|Default|GetLootOutlineComponent))
  (Components|StaticMesh|SetStaticMesh (Variables|Default|GetItem) "/Game/FlexibleCombatSystem/Meshes/General/SM_DropBag.SM_DropBag")
  (Collision|SetCollisionEnabled (Variables|Default|GetItem2) "NoCollision"))

(fn OnRepDroppedLoot
  (CallFunction|InitializeDroppedLoot))

(fn RetrieveInventoryInfo
  (return "NewEnumerator0" "" 0 0 false false 0 0))

(fn RetrieveLootInfo
  (return (Variables|SetupinGame|GetLootSetupInfo)))

(fn RetrieveOutlineInfo
  (bind _lootsetupinfo (Variables|SetupinGame|GetLootSetupInfo))
  (bind (_lootname _rarityoflootcolour) (Utilities|Struct|BreakS_LootSetupInfo _lootsetupinfo))
  (return _lootname _rarityoflootcolour "NewEnumerator1" 0 (Variables|Default|GetItem) (Variables|Default|GetItem2) 0 false))