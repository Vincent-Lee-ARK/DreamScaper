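; Attack hitbox actor that snaps to a socket on a character's mesh for animal or fist melee hits.
; While attacking, locally controlled or AI-tagged characters run a looping owner-scaled sphere trace, tracking hit actors until the attack stops.
; Each new hit triggers a slightly larger server re-trace at that location.
; The server passes damage info to TakingDamage components and applies point damage using WeaponCollision's values.
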(event Custom|AttachToUnit
  (params (CharacterRef :type Character%20Object%20Reference) (SocketName :type Name) (Damage%20Type :type E_DamageType%20Enum :default "NewEnumerator0") (Special%20Damage%20Info :type S%20Special%20Damage%20Info%20Structure))
  ;[1 1 1] Attach Fists To Player
  (bind _output_get (Variables|Default|SetCharacterRef CharacterRef))
  (Actor|SetOwner _output_get)
  (Variables|Default|SetDamage%20Type Damage%20Type)
  (Variables|Default|SetSpecial%20Damage%20Info Special%20Damage%20Info)
  (Variables|Default|SetEquipmentComponent (Actor|GetComponentbyClass _output_get "/Game/FlexibleCombatSystem/Blueprints/Components/EquipmentComponent.EquipmentComponent_C"))
  (Transformation|AttachComponentToComponent (Variables|/Script/Engine.Character|GetMesh (Variables|Default|GetCharacterRef)) SocketName "SnapToTarget" "SnapToTarget" "KeepRelative" true))

(event Custom|Trace
  (bind _returnvalue (Transformation|GetActorLocation))
  ;[1 1 1] Client Sphere Trace
  (bind (_outhits _returnvalue_2) (Collision|MultiSphereTraceForObjects _returnvalue _returnvalue (* (Math|Float|Clamp(Float) (.x (Transformation|GetActorScale3D (Components|GetOwner))) 1.0 3.0) 3e+01) (Utilities|Array|MakeArray "ObjectTypeQuery3") false (Utilities|Array|MakeArray (Variables|Default|GetCharacterRef)) "None"))
  (for _array_element _outhits
    (if _returnvalue_2
      (Utilities|IsValid (Actor|GetComponentbyClass (.HitActor (Collision|BreakHitResult _array_element)) "/Game/FlexibleCombatSystem/Blueprints/Components/TakingDamage.TakingDamage_C")
        (:Is%20Valid
          (if (not (Utilities|Array|ContainsItem (Variables|Default|GetAlreadyDamagedEnemy) (.HitActor (Collision|BreakHitResult _array_element))))
            (Utilities|Array|Add (Variables|Default|GetAlreadyDamagedEnemy) (.HitActor (Collision|BreakHitResult _array_element)))
            (CallFunction|SRCheckHit _returnvalue)))))))

(event Custom|SR_CheckHit
  (params (Start :type Vector))
  (bind _weaponcollision (Variables|Default|GetWeaponCollision))
  ;[1 1 1] We use the Server To Check if the Hit Lands
  (bind (_outhits _returnvalue) (Collision|MultiSphereTraceForObjects Start Start (* (Math|Float|Clamp(Float) (.x (Transformation|GetActorScale3D (Components|GetOwner))) 1.0 3.0) 35.0) (Utilities|Array|MakeArray "ObjectTypeQuery3") false (Utilities|Array|MakeArray (Variables|Default|GetCharacterRef)) "None"))
  (for _array_element _outhits
    (if _returnvalue
      (Utilities|IsValid (Actor|GetComponentbyClass (.HitActor (Collision|BreakHitResult _array_element)) "/Game/FlexibleCombatSystem/Blueprints/Components/TakingDamage.TakingDamage_C")
        (:Is%20Valid
          (Default|PassDamageInfo :self (Actor|GetComponentbyClass (.HitActor (Collision|BreakHitResult _array_element)) "/Game/FlexibleCombatSystem/Blueprints/Components/TakingDamage.TakingDamage_C") :Particle%20System (Variables|/Game/FlexibleCombatSystem/Blueprints/Components/WeaponCollision.WeaponCollision_C|GetWeaponPS _weaponcollision) :AttackType "NewEnumerator17" :Damage%20Type (Variables|Default|GetDamage%20Type) :CriticalHit (Variables|/Game/FlexibleCombatSystem/Blueprints/Components/WeaponCollision.WeaponCollision_C|GetCriticalHit _weaponcollision) :SpecialDamageInfo (Variables|Default|GetSpecial%20Damage%20Info) :Physical%20Anim%20Type "NewEnumerator3")
          (Game|Damage|ApplyPointDamage (.HitActor (Collision|BreakHitResult _array_element)) (Variables|/Game/FlexibleCombatSystem/Blueprints/Components/WeaponCollision.WeaponCollision_C|GetWeaponOutputDamage (Variables|Default|GetWeaponCollision)) (.Location (Collision|BreakHitResult _array_element)) (Collision|MakeHitResult false false 0.0 0.0 "0, 0, 0" (.Location (Collision|BreakHitResult _array_element)) "0,0,1" "0,0,1" 0 0) 0 (Variables|Default|GetCharacterRef)))))))

(event EventStartAttack
  ;[1 1 1] Attack AND Generate LineTrace For Hit - We do this in the Fist and not Weapon Collision because the Fists have 2 traces
  (if (Pawn|IsLocallyControlled (Variables|Default|GetCharacterRef))
    (CallFunction|AttachDamageAttachment)
    (bind _returnvalue (Utilities|Time|SetTimerbyEvent (delegate Custom|Trace) 0.02 true :!label _label))
    (elif (Actor|ActorHasTag (Variables|Default|GetCharacterRef) "AI-Unit")
      (goto _label))))

(event EventStopAttack
  ;[1 1 1] Attack AND Generate LineTrace For Hit - We do this in the Fist and not Weapon Collision because the Fists have 2 traces
  (Utilities|Time|ClearandInvalidateTimerbyHandle (stale EventStartAttack _returnvalue))
  (Utilities|Array|Clear (Variables|Default|GetAlreadyDamagedEnemy)))

(fn ConstructionScript)

(fn LineTraceHit
  (bind _returnvalue (Transformation|GetActorLocation))
  (bind (_outhit _returnvalue_2) (Collision|SphereTraceForObjects _returnvalue _returnvalue 4e+01 (Utilities|Array|MakeArray "ObjectTypeQuery3") false (Utilities|Array|MakeArray (Variables|Default|GetCharacterRef)) "Persistent"))
  (if _returnvalue_2
    (if (not (Utilities|Array|ContainsItem (Variables|Default|GetAlreadyDamagedEnemy) (.HitActor (Collision|BreakHitResult _outhit))))
      (Utilities|Array|Add (Variables|Default|GetAlreadyDamagedEnemy) (.HitActor (Collision|BreakHitResult _outhit)))
      (CallFunction|SRCheckHit _returnvalue))))

(fn AttachDamageAttachment
  (Utilities|FlowControl|DoOnce false))