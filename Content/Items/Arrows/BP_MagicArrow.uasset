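; Magic arrow projectile that takes on an elemental damage type and a matching glow colour when spawned.
; On BeginPlay it finds the owning character's inventory slot data table row, then sets ArrowComponent's damage type and special damage info from that row, or from RangedComponent's ArrowInfo for AI units.
; It then creates dynamic materials on the arrow mesh, tinting them by damage type with high-intensity colours for some elements and black for the rest.
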(event EventBeginPlay
  (bind _arrow (Variables|Default|GetArrow))
  (bind _arrowcomponent (Variables|Default|GetArrowComponent))
  (bind _characterref (Variables|Default|GetCharacterRef))
  (bind _returnvalue (Actor|GetComponentbyClass _characterref "/Game/FlexibleCombatSystem/Blueprints/Components/RangedComponent.RangedComponent_C"))
  (bind _returnvalue_2 (Actor|GetComponentbyClass _characterref "/Game/FlexibleCombatSystem/Blueprints/Components/InventoryComponent.InventoryComponent_C"))
  (bind _slot_number (CallFunction|GetSlotNumber _returnvalue_2 "NewEnumerator13"))
  (bind _arrowinfo (Variables|/Game/FlexibleCombatSystem/Blueprints/Components/RangedComponent.RangedComponent_C|GetArrowInfo _returnvalue))
  (bind _inventorydata (Variables|/Game/FlexibleCombatSystem/Blueprints/Components/InventoryComponent.InventoryComponent_C|GetInventoryData _returnvalue_2))
  (bind _ai_unit (Variables|/Game/FlexibleCombatSystem/Blueprints/Components/RangedComponent.RangedComponent_C|GetAI-Unit _returnvalue))
  (bind _equipmentinfo (Utilities|Struct|BreakS_ItemData _arrowinfo))
  (bind _output (Utilities|Array|Get(acopy) _inventorydata _slot_number))
  (bind _datatableinfo (Utilities|Struct|BreakS_SlotInfo _output))
  (bind (_damagetype _specialdamageinfo) (Utilities|Struct|BreakS_EquipmentInfo _equipmentinfo))
  (bind (_datatable _rowname) (Utilities|Struct|BreakDataTableRowHandle _datatableinfo))
  ;[1 1 1] Retrieve Magic Values
  (Utilities|IsValid _characterref
    (:Is%20Valid
      (bind _returnvalue_3 (Utilities|GetDataTableRow _datatable _rowname)
        (:then
          (Variables|/Game/FlexibleCombatSystem/Blueprints/Components/ArrowComponent.ArrowComponent_C|SetDamageTypeSet _arrowcomponent true)
          (bind _output_get (Variables|/Game/FlexibleCombatSystem/Blueprints/Components/ArrowComponent.ArrowComponent_C|SetDamageType _arrowcomponent (select _ai_unit _damagetype (.DamageType (Utilities|Struct|BreakS_EquipmentInfo (Utilities|Struct|BreakS_ItemData _returnvalue_3))))))
          (Variables|/Game/FlexibleCombatSystem/Blueprints/Components/ArrowComponent.ArrowComponent_C|SetSpecialDamageInfo _arrowcomponent (select _ai_unit _specialdamageinfo (.SpecialDamageInfo (Utilities|Struct|BreakS_EquipmentInfo (Utilities|Struct|BreakS_ItemData _returnvalue_3)))))
          ;[1 1 1] Setup Magic Arrow Materials
          (for (_ _array_index) (Rendering|Material|GetMaterials _arrow)
            (bind _returnvalue_4 (Rendering|Material|CreateDynamicMaterialInstance _arrow _array_index (Rendering|Material|GetMaterial _arrow 0) "None" :!class /Script/Engine.PrimitiveComponent))
            (Rendering|Material|SetScalarParameterValue _returnvalue_4 "Value" 0.1 :!class /Script/Engine.MaterialInstanceDynamic)
            (Rendering|Material|SetVectorParameterValue _returnvalue_4 "Colour" (Utilities|Select :Index _output_get :NewEnumerator0 "" :NewEnumerator1 "(R=300.000000,G=33.448704,B=0.000000,A=1.000000)" :NewEnumerator2 "" :NewEnumerator8 "(R=0.000000,G=242.207047,B=300.000000,A=1.000000)" :NewEnumerator3 "(R=300.000000,G=209.420441,B=0.000000,A=1.000000)" :NewEnumerator4 "(R=97.154366,G=300.000000,B=0.000000,A=1.000000)" :NewEnumerator5 "" :NewEnumerator6 "" :NewEnumerator7 "" :NewEnumerator9 "") :!class /Script/Engine.MaterialInstanceDynamic)))))))

(event Collision|EventActorBeginOverlap
  (params (OtherActor :type Actor%20Object%20Reference)))

(event EventTick
  (params (DeltaSeconds :type Float%20%28single-precision%29))
  (|CallParentFunction DeltaSeconds) ; This node is disabled and will not be called.\nDrag off pins to build functionality.
)

(fn ConstructionScript
  (|CallParentFunction))