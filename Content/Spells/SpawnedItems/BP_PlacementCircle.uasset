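; BP_PlacementCircle is a decal actor that draws a colored circle for spell placement.
; On BeginPlay it applies and scales the decal, creates a dynamic material instance, and sets its color by the spell's element type.
; FadeIn and FadeOut play and reverse a timeline driving the material's opacity, guarded by a flag so repeated calls are ignored.
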(event Custom|FadeIn
  (if (not (Variables|Default|GetFadedIn))
    (Variables|Default|SetFadedIn true)
    (bind _newtrack_0 (Timeline|Fade PlayFromStart)
      (:Update
        (Rendering|Material|SetScalarParameterValue (Variables|Default|GetDecalMaterialInstance) "Opacity" _newtrack_0 :!class /Script/Engine.MaterialInstanceDynamic)))))

(event Custom|FadeOut
  (if (Variables|Default|GetFadedIn)
    (Variables|Default|SetFadedIn false)
    (bind _newtrack_0 (Timeline|Fade ReverseFromEnd)
      (:Update
        (Rendering|Material|SetScalarParameterValue (Variables|Default|GetDecalMaterialInstance) "Opacity" _newtrack_0 :!class /Script/Engine.MaterialInstanceDynamic)))))

(event EventBeginPlay
  (bind _decalsize (Variables|Default|GetDecalSize))
  (Rendering|Components|Decal|SetDecalMaterial (Variables|Default|GetDecal) (Variables|Default|GetDecalMaterial))
  (Transformation|SetRelativeScale3D (Variables|Default|GetDecal) (Math|Vector|MakeVector 5e+02 _decalsize _decalsize))
  (bind _returnvalue (Rendering|Material|CreateDynamicMaterialInstance (Variables|Default|GetDecal) :!class /Script/Engine.DecalComponent))
  (Variables|Default|SetDecalMaterialInstance _returnvalue)
  (Rendering|Material|SetVectorParameterValue (Variables|Default|GetDecalMaterialInstance) "Color" (Utilities|Select :Index (Variables|Default|GetAI%20Spell) :NewEnumerator0 "" :NewEnumerator1 "(R=1.000000,G=0.303948,B=0.000000,A=1.000000)" :NewEnumerator2 "(R=0.000000,G=0.798837,B=1.000000,A=1.000000)" :NewEnumerator8 "(R=0.000000,G=0.138272,B=1.000000,A=1.000000)" :NewEnumerator3 "(R=1.000000,G=0.683297,B=0.000000,A=1.000000)" :NewEnumerator4 "(R=0.133985,G=0.508185,B=0.000000,A=1.000000)" :NewEnumerator5 "(R=1.000000,G=0.000000,B=0.186681,A=1.000000)" :NewEnumerator6 "(R=0.435460,G=0.000000,B=1.000000,A=1.000000)" :NewEnumerator7 "" :NewEnumerator9 "") :!class /Script/Engine.MaterialInstanceDynamic))

(fn ConstructionScript)