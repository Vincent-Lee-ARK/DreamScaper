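; BP_LoweringGate is an activatable gate that slides its Cube downward once when MCInteract fires.
; A DoOnce-guarded timeline lerps the cube, then sets the RepNotify InteractComplete, whose OnRep snaps it to the lowered position.
; InstantActivate skips the animation by setting that flag directly.
; The construction script picks the cube's material from the SystemsTraining flag or the Melee, Ranged or Magic Colour.
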(event EventInstantActivate
  (Variables|Default|SetInteractComplete true))

(event EventMCInteract
  (Utilities|FlowControl|DoOnce false
    (:Completed
      (bind _newtrack_0 (Timeline|Move PlayFromStart)
        (:Update
          (Transformation|SetRelativeLocation (Variables|Default|GetCube) (Math|Vector|Lerp(Vector) "0, 0, 0" "0.000000, 0,-250.000000" _newtrack_0) false false))
        (:Finished
          (Variables|Default|SetInteractComplete true))))))

(fn ConstructionScript
  (if (Variables|Default|GetSystemsTraining)
    (Rendering|Material|SetMaterial (Variables|Default|GetCube) 0 "/Game/FlexibleCombatSystem/DemoFolder/Materials/MI_SystemsTraining.MI_SystemsTraining")
    (else
      (Rendering|Material|SetMaterial (Variables|Default|GetCube) 0 (Utilities|Select :Index (Variables|Default|GetColour) :NewEnumerator0 "/Game/FlexibleCombatSystem/DemoFolder/Materials/MI_MeleeTraining.MI_MeleeTraining" :NewEnumerator1 "/Game/FlexibleCombatSystem/DemoFolder/Materials/MI_RangedTraining.MI_RangedTraining" :NewEnumerator2 "/Game/FlexibleCombatSystem/DemoFolder/Materials/MI_MagicTraining.MI_MagicTraining")))))

(fn OnRepInteractComplete
  (Transformation|SetRelativeLocation (Variables|Default|GetCube) "0.000000,0.000000,-250.000000" false false))