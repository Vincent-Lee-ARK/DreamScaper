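; Box trigger that shows a location discovery widget when the locally controlled player enters and can serve as a quest objective.
; As an objective, it polls until the player is valid, binds to QuestReceiverComponent's objective link, and reports overlaps through IsQuestActor.
; PassObjectiveData sends its position and actor reference to the receiver for matching tracked objectives on the current map.
; PassMapTrackingInfo exposes its map tracking display settings.
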(event OnComponentBeginOverlap(Box)
  (params (OverlappedComponent :type Primitive%20Component%20Object%20Reference) (OtherActor :type Actor%20Object%20Reference) (OtherComp :type Primitive%20Component%20Object%20Reference) (OtherBodyIndex :type Integer) (bFromSweep :type Boolean) (SweepResult :type Hit%20Result%20Structure%20%28by%20ref%29))
  ;[1 1 1] Location Trigger
  (bind _ascharacter (Utilities|Casting|CastToCharacter OtherActor))
  (if (Pawn|IsLocallyControlled _ascharacter)
    (if (Actor|ActorHasTag OtherActor "Player")
      (bind _returnvalue (UserInterface|CreateWidget "/Game/FlexibleCombatSystem/Widgets/General/WB_LocationDiscover.WB_LocationDiscover_C" 0 (Variables|Setup|GetLocationName)))
      (UserInterface|Viewport|AddtoViewport _returnvalue 0)
      (if (Variables|Setup|GetQuestObjective?)
        (CallFunction|IsQuestActor (Game|GetPlayerCharacter 0) (Variables|Setup|GetLocationName) 1 (Transformation|GetActorLocation) (Utilities|GetObjectName self))))))

(event Custom|PlayerValidCheck
  ;[1 1 1] Bind Quest Objective Link
  (Utilities|IsValid (Game|GetPlayerCharacter 0)
    (:Is%20Valid
      (Utilities|Time|ClearandInvalidateTimerbyHandle (stale EventBeginPlay _returnvalue))
      (EventDispatchers|BindEventtoQuestObjectiveLink (Actor|GetComponentbyClass (Game|GetPlayerCharacter 0) "/Game/FlexibleCombatSystem/Blueprints/Components/QuestReceiverComponent.QuestReceiverComponent_C") (EventDispatchers|CreateEvent :!event PassObjectiveData)))))

(event EventBeginPlay
  ;[1 1 1] Bind Quest Objective Link
  (if (Variables|Setup|GetQuestObjective?)
    (CallFunction|PlayerValidCheck)
    (bind _returnvalue (Utilities|Time|SetTimerbyEvent (delegate Custom|PlayerValidCheck) 0.5 true))))

(fn ConstructionScript)

(fn PassObjectiveData
  (params (Quest%20Receiver :type Quest%20Receiver%20Component%20Object%20Reference) (Quest%20Info :type S%20Quest%20Info%20Structure))
  ;[1 1 1] IF Quest Item is Part of Quest Pass Data (Updated Location) over to Quest Log
  (bind (_array_element _array_index) (Utilities|Array|ForEachLoopwithBreak (.QuestObjectiveInfo (Utilities|Struct|BreakS_QuestInfo Quest%20Info)) :!label _label)
    (:LoopBody
      (if (Utilities|Enum|Equal(Enum) (Variables|Setup|GetLocationName) (.ObjectiveName (Utilities|Struct|BreakS_QuestObjectiveInfo _array_element)))
        (if (.ObjectiveHasTracking? (Utilities|Struct|BreakS_QuestObjectiveInfo _array_element))
          (bind _returnvalue (Game|GetCurrentLevelName true))
          (if (Utilities|Enum|Equal(Enum) _returnvalue (.ObjectiveMapName (Utilities|Struct|BreakS_QuestObjectiveInfo _array_element)))
            (Default|PassObjectiveUpdatedLocation Quest%20Receiver (Utilities|Struct|MakeS_QuestObjectiveInfo (.ObjectiveName (Utilities|Struct|BreakS_QuestObjectiveInfo _array_element)) "" (.ObjectiveType (Utilities|Struct|BreakS_QuestObjectiveInfo _array_element)) (.TotalObjectiveNumber (Utilities|Struct|BreakS_QuestObjectiveInfo _array_element)) (.ObjectiveHasTracking? (Utilities|Struct|BreakS_QuestObjectiveInfo _array_element)) (.ObjectiveMapName (Utilities|Struct|BreakS_QuestObjectiveInfo _array_element)) (Transformation|GetActorLocation) self) _array_index)
            (goto _label Break)))))))

(fn PassMapTrackingInfo
  (return (Variables|Setup|GetObjectiveTrackingType) (Variables|Setup|GetObjectiveTrackDistance) (Variables|Setup|GetObjectiveTexture) (Variables|Setup|GetObjectiveTextureSize)))