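; BP_ChangeLevel is a trigger actor that sends the player to a named level and shows that destination on a text render.
; When a "Player"-tagged actor enters the overlap, it messages the GameMode to update the "Autosave" slot with the target map and save.
; It then passes spawn settings (player start or specific transform) to the GameMode before opening the level by name.
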(event OnComponentBeginOverlap(ChangeOverlap)
  (params (OverlappedComponent :type Primitive%20Component%20Object%20Reference) (OtherActor :type Actor%20Object%20Reference) (OtherComp :type Primitive%20Component%20Object%20Reference) (OtherBodyIndex :type Integer) (bFromSweep :type Boolean) (SweepResult :type Hit%20Result%20Structure%20%28by%20ref%29))
  (bind _returnvalue (Game|GetGameMode))
  ;[1 1 1] Call This Everytime You Change Levels
  (if (Actor|ActorHasTag OtherActor "Player")
    (Class|IGameMode|UpdateSaveSlot(Message) _returnvalue "Autosave" (Utilities|String|ToString(Name) (Variables|Default|GetLevel%20Name)))
    (Class|IGameMode|SaveGame(Message) _returnvalue)
    (Class|IGameMode|UpdateSpawnLocation(Message) _returnvalue (Variables|Default|GetSpawn%20at%20Player%20Start) (Variables|Default|GetSpawn%20Specific%20Transform))
    (Game|OpenLevel(byName) (Variables|Default|GetLevel%20Name))))

(event EventBeginPlay
  (Rendering|Components|TextRender|SetText (Variables|Default|GetTextRender) (Utilities|Text|ToText(String) (Utilities|String|Append (Utilities|String|MakeLiteralString "Travel to ") (Utilities|String|ToString(Name) (Variables|Default|GetLevel%20Name))))))

(fn ConstructionScript)