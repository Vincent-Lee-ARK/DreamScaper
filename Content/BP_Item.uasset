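; Holdable item that can be picked up, dropped and used, with only debug prints for its primary use so far.
; PickUp disables the Sphere's collision and attaches to the given parent component at the ItemSocket_r socket.
; Drop detaches the Sphere, restores collision, enables physics and applies a fixed world-space force to toss it.
; UsePrimary is a stub noted as triggered by ThirdPersonCharacter on left mouse click.
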(event Custom|PickUp
  (params (ParentActor :type Actor%20Object%20Reference) (Parent :type Scene%20Component%20Object%20Reference))
  (Development|PrintString "PickUp")
  (Collision|SetCollisionEnabled (Variables|Default|GetSphere) "NoCollision")
  (Transformation|AttachComponentToComponent Parent "ItemSocket_r" "SnapToTarget" "SnapToTarget" "KeepRelative" true))

(event Custom|Drop
  (Development|PrintString "Drop")
  (Transformation|DetachFromComponent (Variables|Default|GetSphere) "KeepWorld" "KeepWorld" "KeepRelative" true)
  (Collision|SetCollisionEnabled (Variables|Default|GetSphere) "QueryAndPhysics")
  (Physics|SetSimulatePhysics (Variables|Default|GetSphere) true)
  (Physics|AddForce (Variables|Default|GetSphere) "300.000000,300.000000,300.000000" "None" false))

(event Custom|UsePrimary
  (params (HeldDown :type Boolean))
  (Development|PrintString "PrimaryFire"))

(fn ConstructionScript)