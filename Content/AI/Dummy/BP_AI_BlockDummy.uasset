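; AI block dummy that draws its weapon and keeps blocking, with a raised health pool.
; The ServerActivateAI event initializes components, sets weapon style and health, then starts a looping timer.
; Each tick of that timer re-triggers the melee block and shows the health HUD only while the first player is nearby.
; Setting UpdateAnim drives an OnRep that applies the combat AnimBP from AI setup data.
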(event Custom|Block
  ;[1 1 1] Remove AI Controller (Update Wep BC Controller handles that), Draw Weapon & Block
  (Default|SRBeginBlock (Variables|Default|GetMeleeComponent))
  (bind _asbp_player_character (Utilities|Casting|CastToBP_PlayerCharacter (Game|GetPlayerCharacter 0)))
  (Development|SetHiddeninGame (Variables|Default|GetHealthHUD) (not (< (Transformation|GetDistanceTo _asbp_player_character self) 1e+03)) false))

(event EventBeginPlay
  (|CallParentFunction) ; This node is disabled and will not be called.\nDrag off pins to build functionality.
)

(event EventServerActivateAI
  (bind _equipmentcomponent (Variables|Default|GetEquipmentComponent))
  ;[1 1 1] Remove AI Controller (Update Wep BC Controller handles that), Draw Weapon & Block
  ;;[1 1 1] Remove functionality
  (CallFunction|MCInitializeComponents)
  (Default|UpdateWeaponStyle (Variables|Default|GetCombatStatusComponent) "NewEnumerator6")
  (Variables|Default|SetUpdateAnim true)
  (Variables|/Game/FlexibleCombatSystem/Blueprints/Components/EquipmentComponent.EquipmentComponent_C|SetHealth _equipmentcomponent 1e+03)
  (Variables|/Game/FlexibleCombatSystem/Blueprints/Components/EquipmentComponent.EquipmentComponent_C|SetMaxHealth _equipmentcomponent 1e+03)
  (Default|OwningClientRPC _equipmentcomponent "NewEnumerator1" false)
  (Default|SRDrawWeapon (Variables|Default|GetCombatStatusComponent))
  (Utilities|Time|SetTimerbyEvent (delegate Custom|Block) 3.0 true))

(fn ConstructionScript
  (|CallParentFunction))

(fn OnRepUpdateAnim
  (bind _mesh (Variables|Character|GetMesh))
  (Class|SkeletalMeshComponent|SetAnimClass _mesh (Utilities|Struct|BreakS_AI-CombatData (.CombatData (Utilities|Struct|BreakS_AI-Data (CallFunction|GetAIData (Variables|Default|GetAI%20Setup%20Data))))))
  (Class|IAI-ABP|SetupAI-ABP(Message) (Components|SkeletalMesh|GetAnimInstance _mesh)))