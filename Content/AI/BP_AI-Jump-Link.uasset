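; A placeable smart nav link that makes AI characters jump to the link's destination.
; On arrival it pauses the agent's brain logic and launches it on a ballistic arc solved from a set leap duration and hard-coded gravity.
; Tick yaws the character toward the landing point until the delay ends and logic restarts.
; A gate flag allows one jumper at a time, halting others' movement without queuing them.
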(event EventTick
  (params (DeltaSeconds :type Float%20%28single-precision%29))
  (bind _character (Variables|Default|GetCharacter))
  (bind _returnvalue (Transformation|GetActorRotation _character))
  (bind (_roll _pitch) (Math|Rotator|BreakRotator _returnvalue))
  ;[1 1 1] Rotate
  (Transformation|SetActorRotation (Variables|Default|GetCharacter) (Math|Rotator|MakeRotator _roll _pitch (.yaw (Math|Interpolation|RInterpTo _returnvalue (Math|Rotator|FindLookatRotation (Transformation|GetActorLocation _character) (Variables|Default|GetEndLocation)) DeltaSeconds 1e+01)))))

(event EventSmartLinkReached
  (params (Agent :type Actor%20Object%20Reference) (Destination :type Vector%20%28by%20ref%29 :default "0, 0, 0"))
  (bind _leap_duration (Variables|Default|GetLeap%20Duration))
  ;[1 1 1] This is the Tool used to get your AI to Jump. To set it up place it in the Level
  (if (Variables|Default|GetGateInUse)
    (AI|Navigation|StopMovement (AI|GetAIController Agent))
    (else
      (Variables|Default|SetGateInUse true)
      (Variables|Default|SetCharacter Agent)
      (Variables|Default|SetEndLocation Destination)
      (AI|Logic|StopLogic (Variables|/Script/AIModule.AIController|GetBrainComponent (AI|GetAIController (Variables|Default|GetCharacter))) "")
      (bind _velocity (CallFunction|CalculateLeapVelocity (Transformation|GetActorLocation) (Variables|Default|GetEndLocation) _leap_duration))
      (bind _ascharacter (Utilities|Casting|CastToCharacter (Variables|Default|GetCharacter)))
      (Character|LaunchCharacter _ascharacter _velocity true true)
      (Actor|Tick|SetActorTickEnabled true)
      (Utilities|FlowControl|Delay _leap_duration)
      (AI|Logic|StartLogic (Variables|/Script/AIModule.AIController|GetBrainComponent (AI|GetAIController (Variables|Default|GetCharacter))))
      (Actor|Tick|SetActorTickEnabled false)
      (Variables|Default|SetGateInUse false))))

(fn ConstructionScript)

(fn CalculateLeapVelocity
  (params (Start%20Location :type Vector) (Destination :type Vector) (Leap%20Duration :type Float%20%28single-precision%29))
  (bind (_x _y _z) (Math|Vector|BreakVector Start%20Location))
  (bind (_x_2 _y_2 _z_2) (Math|Vector|BreakVector Destination))
  (LocalVariables|SetDuration Leap%20Duration)
  (return (Math|Vector|MakeVector (/ (- _x_2 _x) (LocalVariables|GetDuration)) (/ (- _y_2 _y) (LocalVariables|GetDuration)) (/ (- _z_2 (+ _z (* (Math|Float|Square (LocalVariables|GetDuration)) -0.5 9.8e+02))) (LocalVariables|GetDuration)))))