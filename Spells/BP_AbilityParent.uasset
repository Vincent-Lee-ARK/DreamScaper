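; Base spell Blueprint that declares the ability lifecycle: initialize, charge, channel release, fire on anim notify, load from save, and destroy.
; Most bodies are empty stubs, including placement marker, velocity and hit-location functions, plus authority checks and RepNotifies for networking.
; The one working calculation, GetCameraPlayerLevel, projects the character's control direction from the camera position by the camera-to-character distance.
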(event Custom|BeginMagicCharge
  ;[1 1 1] Begin Charge - Called When Spell Created
)

(event Custom|StopMagicCharge
  ;[1 1 1] Stop Magic Charge - Called When Spell Released
)

(event Custom|MC_Initialize
  (params (SpellInfo :type Data%20Table%20Row%20Handle%20Structure) (NiagaraNS :type Niagara%20System%20Object%20Reference) (CharacterRef :type Character%20Object%20Reference))
  ;[1 1 1] Setup & Initialize
)

(event Custom|SendMagicSpell
  ;[1 1 1] Send Magic Spell - Called When Spell Tries To Fire
)

(event Custom|TriggerMagicSpell
  ;[1 1 1] Trigger Magic Spell - Called when Anim Notify Fires Spell
)

(event Custom|ReleaseSpellChannel
  ;[1 1 1] Release Spell Channel - Called When Left MB Released
)

(event Custom|ClearSpellPlacement)

(event Custom|Initialize
  (params (SpellInfo :type Data%20Table%20Row%20Handle%20Structure) (NiagaraSystem :type Niagara%20System%20Object%20Reference) (CharacterRef :type Character%20Object%20Reference))
  ;[1 1 1] Setup & Initialize
)

(event Custom|LoadSpell
  (params (TimeRemaining :type Float%20%28double-precision%29))
  ;[1 1 1] Load Spell - Called When Spell Load Game Creates Spells Again
)

(event Custom|DestroySpell
  ;[1 1 1] Destroy Self - Called When Spell Getting Destroyed
)

(fn ConstructionScript)

(fn UpdateSpellPlacement
  ;[1 1 1] Sets Marker For Spell Placement
)

(fn CalculateSpellVelocity)

(fn GetCameraRelative)

(fn GetCameraLocation)

(fn GetCameraForward
  (if (Variables|Default|GetAI_Spell)
    (return "0, 0, 0")
    (else
      (return "0, 0, 0"))))

(fn GetCameraPlayerLevel
  (bind _camerarelative (CallFunction|GetCameraRelative))
  (bind _characterref (Variables|References|GetCharacterRef))
  (bind _returnvalue (Transformation|GetActorLocation _characterref))
  (bind _returnvalue_2 (+ _camerarelative _returnvalue))
  (return (+ (* (Math|Vector|GetForwardVector (Pawn|GetControlRotation (Variables|References|GetCharacterRef) :!class /Script/Engine.Pawn)) (Math|Vector|VectorLength (- (Transformation|GetActorLocation _characterref) _returnvalue_2))) _returnvalue_2)))

(fn SetupVariables&References)

(fn RemovePlacementMarker)

(fn Spell-Interupted)

(fn CalculateSpellHitLocation)

(fn OnRepActivated)

(fn SpellFiredAuthorityORLocal)

(fn ActivateNS)

(fn CorrectAuthority)

(fn OnRepSpellVelocity)