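; Parent item Blueprint for consumables such as potions that restore the character's health, stamina or mana.
; ConsumeonUse runs the flow on the server and calls OCConsume for non-local characters, reading type and power from item data.
; After an animation-based delay, restore functions add clamped values under authority, show combat text and trigger resource updates.
; A random drink sound then plays and the authority destroys the actor; ActivateBuff is an empty stub.
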(event Custom|OC_Consume
  (bind _iteminfo (Variables|Default|GetItemInfo))
  (bind _datatableinfo (Utilities|Struct|BreakS_SlotInfo _iteminfo))
  (bind _slotdata (CallFunction|GetItemData _datatableinfo))
  (bind _consumableinfo (Utilities|Struct|BreakS_ItemData _slotdata))
  (bind (_consumablepower _consumableduration) (Utilities|Struct|BreakS_ConsumableInfo _consumableinfo))
  ;[1 1 1] Consumable Usage
  (Variables|Default|SetConsumable%20Power _consumablepower)
  (Variables|Default|SetConsumable%20Duration _consumableduration)
  (Variables|Default|SetBuffComponent (Actor|GetComponentbyClass (Variables|Default|GetCharacterRef) "/Game/FlexibleCombatSystem/Blueprints/Components/BuffComponent.BuffComponent_C"))
  (bind _output_get (Variables|Default|SetConsumable%20Type (Utilities|Struct|BreakS_ConsumableInfo (Utilities|Struct|BreakS_ItemData (CallFunction|GetItemData (Utilities|Struct|BreakS_SlotInfo (Variables|Default|GetItemInfo)))))))
  (Utilities|FlowControl|Delay (- (Variables|Default|GetConsumeAnimLength) 2.0))
  (switch Utilities|FlowControl|Switch|SwitchonE_ConsumableType _output_get
    (:NewEnumerator0
      (CallFunction|RestoreHealth))
    (:NewEnumerator1
      (CallFunction|RestoreStamina))
    (:NewEnumerator2
      (CallFunction|RestoreMana)))
  ;[1 1 1] Animation Finish, Destroy
  (Audio|PlaySoundatLocation (.OutItem (Utilities|Array|Random (Utilities|Array|MakeArray (CallFunction|PassSoundFX "DrinkPotion1") (CallFunction|PassSoundFX "DrinkPotion2")))) (Transformation|GetActorLocation (Variables|Default|GetCharacterRef)) "0, 0, 0" 1.0 1.0 0.0 0 0 0 0)
  (Utilities|FlowControl|Delay 1.5)
  (Networking|SwitchHasAuthority
    (:Authority
      (Actor|DestroyActor))))

(event EventConsumeonUse
  (bind _iteminfo (Variables|Default|GetItemInfo))
  (bind _datatableinfo (Utilities|Struct|BreakS_SlotInfo _iteminfo))
  (bind _slotdata (CallFunction|GetItemData _datatableinfo))
  (bind _consumableinfo (Utilities|Struct|BreakS_ItemData _slotdata))
  (bind (_consumablepower _consumableduration) (Utilities|Struct|BreakS_ConsumableInfo _consumableinfo))
  ;[1 1 1] Consumable Usage
  ;;[1 1 1] Currently Running on just Server, ignore send to Client if Standalone
  (if (Pawn|IsLocallyControlled (Variables|Default|GetCharacterRef))
    _
    (else
      (CallFunction|OCConsume)))
  (Variables|Default|SetConsumable%20Power _consumablepower)
  (Variables|Default|SetConsumable%20Duration _consumableduration)
  (Variables|Default|SetBuffComponent (Actor|GetComponentbyClass (Variables|Default|GetCharacterRef) "/Game/FlexibleCombatSystem/Blueprints/Components/BuffComponent.BuffComponent_C"))
  (bind _output_get (Variables|Default|SetConsumable%20Type (Utilities|Struct|BreakS_ConsumableInfo (Utilities|Struct|BreakS_ItemData (CallFunction|GetItemData (Utilities|Struct|BreakS_SlotInfo (Variables|Default|GetItemInfo)))))))
  (Utilities|FlowControl|Delay (- (Variables|Default|GetConsumeAnimLength) 2.0))
  (switch Utilities|FlowControl|Switch|SwitchonE_ConsumableType _output_get
    (:NewEnumerator0
      (CallFunction|RestoreHealth))
    (:NewEnumerator1
      (CallFunction|RestoreStamina))
    (:NewEnumerator2
      (CallFunction|RestoreMana)))
  ;[1 1 1] Animation Finish, Destroy
  (Audio|PlaySoundatLocation (.OutItem (Utilities|Array|Random (Utilities|Array|MakeArray (CallFunction|PassSoundFX "DrinkPotion1") (CallFunction|PassSoundFX "DrinkPotion2")))) (Transformation|GetActorLocation (Variables|Default|GetCharacterRef)) "0, 0, 0" 1.0 1.0 0.0 0 0 0 0)
  (Utilities|FlowControl|Delay 1.5)
  (Networking|SwitchHasAuthority
    (:Authority
      (Actor|DestroyActor))))

(fn ConstructionScript
  (|CallParentFunction))

(fn ActivateBuff)

(fn RestoreHealth
  (bind _equipmentcomponent (Variables|Default|GetEquipmentComponent))
  (bind _maxhealth (Variables|/Game/FlexibleCombatSystem/Blueprints/Components/EquipmentComponent.EquipmentComponent_C|GetMaxHealth _equipmentcomponent))
  ;[1 1 1] Increase Health
  (Networking|SwitchHasAuthority
    (:Authority
      (bind _output_get (Variables|/Game/FlexibleCombatSystem/Blueprints/Components/EquipmentComponent.EquipmentComponent_C|SetHealth _equipmentcomponent (+ (Variables|/Game/FlexibleCombatSystem/Blueprints/Components/EquipmentComponent.EquipmentComponent_C|GetHealth _equipmentcomponent) (Variables|Default|GetConsumable%20Power))))
      ;;[1 1 1] Set Health Back To Max Health If Goes Above
      (if (> _output_get _maxhealth)
        (Variables|/Game/FlexibleCombatSystem/Blueprints/Components/EquipmentComponent.EquipmentComponent_C|SetHealth _equipmentcomponent _maxhealth)))
    (:Remote
      _))
  (bind _returnvalue (UserInterface|CreateWidget "/Game/FlexibleCombatSystem/Widgets/Combat/WB_CombatText.WB_CombatText_C" 0 (Transformation|GetActorLocation (Variables|Default|GetCharacterRef)) (Math|Float|Round (Variables|Default|GetConsumable%20Power)) "NewEnumerator13"))
  (Utilities|IsValid _returnvalue
    (:Is%20Valid
      (UserInterface|Viewport|AddtoViewport _returnvalue 0))
    (:Is%20Not%20Valid
      _))
  (Default|OwningClientRPC (Variables|Default|GetEquipmentComponent) "NewEnumerator6" false))

(fn RestoreStamina
  (bind _equipmentcomponent (Variables|Default|GetEquipmentComponent))
  (bind _maxstamina (Variables|/Game/FlexibleCombatSystem/Blueprints/Components/EquipmentComponent.EquipmentComponent_C|GetMaxStamina _equipmentcomponent))
  ;[1 1 1] Restore Stamina
  (Networking|SwitchHasAuthority
    (:Authority
      (bind _output_get (Variables|/Game/FlexibleCombatSystem/Blueprints/Components/EquipmentComponent.EquipmentComponent_C|SetStamina _equipmentcomponent (+ (Variables|/Game/FlexibleCombatSystem/Blueprints/Components/EquipmentComponent.EquipmentComponent_C|GetStamina _equipmentcomponent) (Variables|Default|GetConsumable%20Power))))
      ;;[1 1 1] Set Stamina Back To Max Stamina If Goes Above
      (if (> _output_get _maxstamina)
        (Variables|/Game/FlexibleCombatSystem/Blueprints/Components/EquipmentComponent.EquipmentComponent_C|SetStamina _equipmentcomponent _maxstamina)))
    (:Remote
      _))
  (bind _returnvalue (UserInterface|CreateWidget "/Game/FlexibleCombatSystem/Widgets/Combat/WB_CombatText.WB_CombatText_C" 0 (Transformation|GetActorLocation (Variables|Default|GetCharacterRef)) (Math|Float|Round (Variables|Default|GetConsumable%20Power)) "NewEnumerator13"))
  (Utilities|IsValid _returnvalue
    (:Is%20Valid
      (UserInterface|Viewport|AddtoViewport _returnvalue 0))
    (:Is%20Not%20Valid
      _))
  (Default|UpdateStaminaDispatch (Actor|GetComponentbyClass (Variables|Default|GetCharacterRef) "/Game/FlexibleCombatSystem/Blueprints/Components/ResourceComponent.ResourceComponent_C")))

(fn RestoreMana
  (bind _equipmentcomponent (Variables|Default|GetEquipmentComponent))
  (bind _maxmana (Variables|/Game/FlexibleCombatSystem/Blueprints/Components/EquipmentComponent.EquipmentComponent_C|GetMaxMana _equipmentcomponent))
  ;[1 1 1] Restore Mana
  (Networking|SwitchHasAuthority
    (:Authority
      (bind _output_get (Variables|/Game/FlexibleCombatSystem/Blueprints/Components/EquipmentComponent.EquipmentComponent_C|SetMana _equipmentcomponent (+ (Variables|/Game/FlexibleCombatSystem/Blueprints/Components/EquipmentComponent.EquipmentComponent_C|GetMana _equipmentcomponent) (Variables|Default|GetConsumable%20Power))))
      ;;[1 1 1] Set Mana Back To Max Mana If Goes Above
      (if (> _output_get _maxmana)
        (Variables|/Game/FlexibleCombatSystem/Blueprints/Components/EquipmentComponent.EquipmentComponent_C|SetMana _equipmentcomponent _maxmana)))
    (:Remote
      _))
  (bind _returnvalue (UserInterface|CreateWidget "/Game/FlexibleCombatSystem/Widgets/Combat/WB_CombatText.WB_CombatText_C" 0 (Transformation|GetActorLocation (Variables|Default|GetCharacterRef)) (Math|Float|Round (Variables|Default|GetConsumable%20Power)) "NewEnumerator13"))
  (Utilities|IsValid _returnvalue
    (:Is%20Valid
      (UserInterface|Viewport|AddtoViewport _returnvalue 0))
    (:Is%20Not%20Valid
      _))
  (Default|OwningClientRPC (Variables|Default|GetEquipmentComponent) "NewEnumerator5" false))