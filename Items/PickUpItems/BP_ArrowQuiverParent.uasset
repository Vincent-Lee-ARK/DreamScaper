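; Base Blueprint for arrow quiver pickup items, defining the shared functions and events for loading, passing, counting and resetting arrows.
; Nearly all of them are empty stubs or return defaults, presumably for child quivers to override.
; The implemented getters derive the arrow count from total minus available slots, take the name from item data and quantity from the EquipmentComponent's ammo info, and return self as the quiver reference.
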(event EventDestroySelf&Attachments)

(event EventBeginPlay)

(event EventPlayerDied)

(event EventLowerArrowQuantity)

(event EventLoadArrows)

(event EventIncreaseArrowNumber
  (params (Quantity :type Integer)))

(fn ConstructionScript
  (|CallParentFunction))

(fn SpawnArrowsIntoQuiver)

(fn PassArrow)

(fn ResetSingleArrow
  (params (Target :type Actor%20Object%20Reference)))

(fn RemoveArrowData)

(fn IncreaseArrowQuantity
  (params (New%20Arrows :type Integer)))

(fn LoadSlots)

(fn SetSlot
  (params (Index :type Integer) (SlotTaken :type Boolean) (ArrowRef :type BP%20Arrow%20Parent%20Object%20Reference)))

(fn ContainsArrow
  (return false))

(fn GetArrowType
  (return 0))

(fn ArrowsinQuiver
  (return (- (Variables|Default|GetTotalArrowSlots) (Variables|Default|GetAvailableArrowSlots))))

(fn GetArrowName&Quantity
  (return (.Name (Utilities|Struct|BreakS_ItemData (CallFunction|GetItemData (Utilities|Struct|BreakS_SlotInfo (Variables|Default|GetItemInfo))))) (.quantity (Variables|/Game/FlexibleCombatSystem/Blueprints/Components/EquipmentComponent.EquipmentComponent_C|GetAmmoQuiverInfo (Variables|Default|GetEquipmentComponent)))))

(fn GetBowAttachments
  (return 0 0 0 0 0))

(fn GetQuiverRef
  (return self))

(fn PassArrowRef
  (return 0))