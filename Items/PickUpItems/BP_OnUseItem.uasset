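; Item use handler Blueprint that runs an item-specific effect when a pickup item is used.
; On use, it looks up the item's data table name and maps it to an OnUseItemType, then switches on that type.
; Currently only Campfire is handled, spawning a BP_CraftingCooking station in front of the character and destroying this actor.
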(event EventUseItemonUse
  (CallFunction|DetermineonUseItem)
  (switch Utilities|FlowControl|Switch|SwitchonE_OnUseItemType (Variables|Default|GetOnUseItemType)
    (:NewEnumerator0
      (CallFunction|CampfireonUse))))

(fn ConstructionScript
  (|CallParentFunction))

(fn DetermineonUseItem
  (if (Utilities|Enum|Equal(Enum) (.Name (Utilities|Struct|BreakS_ItemData (CallFunction|GetItemData (Utilities|Struct|BreakS_SlotInfo (Variables|Default|GetItemInfo))))) (Utilities|Text|MakeLiteralText "Campfire"))
    (Variables|Default|SetOnUseItemType "NewEnumerator0")))

(fn CampfireonUse
  (bind _characterref (Variables|Default|GetCharacterRef))
  (Game|SpawnActorfromClass :Class "/Game/FlexibleCombatSystem/Blueprints/Crafting/BP_CraftingCooking.BP_CraftingCooking_C" :SpawnTransform (Math|Transform|MakeTransform (+ (.location (Transformation|GetWorldTransform (Variables|/Script/Engine.Character|GetMesh _characterref))) (* (Transformation|GetActorForwardVector _characterref) 100)) "0, 0, 0" "1,1,1") :CollisionHandlingOverride "Undefined" :Instigator 0)
  (Actor|DestroyActor))