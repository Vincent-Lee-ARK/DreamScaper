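; Unarmed fist weapon that attaches two fist components to the owning character's hand sockets and deals melee damage.
; During attacks, locally controlled or AI-tagged characters run a looping timer that sphere-traces both fists, ignoring already-hit actors until the attack stops.
; The server re-traces each hit, passes attack info to the target's TakingDamage component and applies WeaponCollision damage.
; A hand-built HitResult works around incorrect UE5 impact locations.
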(event Custom|AttachToPlayer
  (params (CharacterRef :type Character%20Object%20Reference))
  ;[1 1 1] Attach Fists To Player
  (bind _output_get (Variables|Default|SetCharacterRef CharacterRef))
  (Actor|SetOwner _output_get)
  (Variables|Default|SetEquipmentComponent (Actor|GetComponentbyClass _output_get "/Game/FlexibleCombatSystem/Blueprints/Components/EquipmentComponent.EquipmentComponent_C"))
  (CallFunction|AttachFists))

(event Custom|Trace
  ;[1 1 1] Attack AND Generate LineTrace For Hit - We do this in the Fist and not Weapon Collision because the Fists have 2 traces
  (CallFunction|LineTraceHit (Variables|Default|GetFist1Ref))
  (CallFunction|LineTraceHit (Variables|Default|GetFist2Ref)))

(event Custom|SR_CheckHit
  (params (Start :type Vector))
  (bind _weaponcollision (Variables|Default|GetWeaponCollision))
  ;[1 1 1] We use the Server To Check if the Hit Lands
  (bind _outhit (Collision|SphereTraceForObjects Start Start 2e+01 (Utilities|Array|MakeArray "ObjectTypeQuery3") false (Utilities|Array|MakeArray (Variables|Default|GetCharacterRef)) "None"))
  (Utilities|IsValid (Actor|GetComponentbyClass (.HitActor (Collision|BreakHitResult _outhit)) "/Game/FlexibleCombatSystem/Blueprints/Components/TakingDamage.TakingDamage_C")
    (:Is%20Valid
      (Default|PassDamageInfo :self (Actor|GetComponentbyClass (.HitActor (Collision|BreakHitResult _outhit)) "/Game/FlexibleCombatSystem/Blueprints/Components/TakingDamage.TakingDamage_C") :Particle%20System (Variables|/Game/FlexibleCombatSystem/Blueprints/Components/WeaponCollision.WeaponCollision_C|GetWeaponPS _weaponcollision) :AttackType "NewEnumerator17" :CriticalHit (Variables|/Game/FlexibleCombatSystem/Blueprints/Components/WeaponCollision.WeaponCollision_C|GetCriticalHit _weaponcollision) :Physical%20Anim%20Type "NewEnumerator3")
      ;;[0.3211 1 0.9359] Bug in UE5 means that the default Hit Info doesn't give the correct Impact Location. Tweaked this to work for UE5, UE4 can plug Normal Hit Info in
      (Game|Damage|ApplyPointDamage (.HitActor (Collision|BreakHitResult _outhit)) (Variables|/Game/FlexibleCombatSystem/Blueprints/Components/WeaponCollision.WeaponCollision_C|GetWeaponOutputDamage (Variables|Default|GetWeaponCollision)) (.Location (Collision|BreakHitResult _outhit)) (Collision|MakeHitResult false false 0.0 0.0 "0, 0, 0" (.Location (Collision|BreakHitResult _outhit)) "0,0,1" "0,0,1" 0 0) 0 (Variables|Default|GetCharacterRef)))))

(event EventStartAttack
  ;[1 1 1] Attack AND Generate LineTrace For Hit - We do this in the Fist and not Weapon Collision because the Fists have 2 traces
  (if (Pawn|IsLocallyControlled (Variables|Default|GetCharacterRef))
    (CallFunction|AttachFists)
    (bind _returnvalue (Utilities|Time|SetTimerbyEvent (delegate Custom|Trace) 0.01 true :!label _label))
    (elif (Actor|ActorHasTag (Variables|Default|GetCharacterRef) "AI-Unit")
      (goto _label))))

(event EventStopAttack
  ;[1 1 1] Attack AND Generate LineTrace For Hit - We do this in the Fist and not Weapon Collision because the Fists have 2 traces
  (Utilities|Time|ClearandInvalidateTimerbyHandle (stale EventStartAttack _returnvalue))
  (Utilities|Array|Clear (Variables|Default|GetAlreadyDamagedEnemy)))

(fn ConstructionScript)

(fn LineTraceHit
  (params (Fist :type Scene%20Component%20Object%20Reference))
  (bind _returnvalue (Transformation|GetWorldLocation Fist))
  (bind (_outhit _returnvalue_2) (Collision|SphereTraceForObjects _returnvalue (Transformation|GetWorldLocation Fist) 2e+01 (Utilities|Array|MakeArray "ObjectTypeQuery3") false (Utilities|Array|MakeArray (Variables|Default|GetCharacterRef)) "None"))
  (if _returnvalue_2
    (if (not (Utilities|Array|ContainsItem (Variables|Default|GetAlreadyDamagedEnemy) (.HitActor (Collision|BreakHitResult _outhit))))
      (Utilities|Array|Add (Variables|Default|GetAlreadyDamagedEnemy) (.HitActor (Collision|BreakHitResult _outhit)))
      (CallFunction|SRCheckHit _returnvalue))))

(fn AttachFists
  (bind _characterref (Variables|Default|GetCharacterRef))
  (bind _mesh (Variables|/Script/Engine.Character|GetMesh _characterref))
  (Utilities|FlowControl|DoOnce false
    (:Completed
      (Transformation|AttachComponentToComponent (Variables|Default|GetFist1Ref) _mesh "hand_L" "SnapToTarget" "SnapToTarget" "KeepRelative" true)
      (Transformation|AttachComponentToComponent (Variables|Default|GetFist2Ref) _mesh "hand_R" "SnapToTarget" "SnapToTarget" "KeepRelative" true))))