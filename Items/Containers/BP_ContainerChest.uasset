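; Chest container Blueprint that animates opening and closing, extending a parent container class.
; ToggleAnimation calls the parent, stores the Scene component's current rotation, then plays or reverses the ToggleChest timeline based on Open.
; Timeline updates lerp Scene along the shortest path, with Open selecting endpoints between the stored rotation and a fixed open or zero closed angle.
; RetrieveLootInfo is empty, and the construction script only calls the parent.
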(event EventToggleAnimation
  ;[1 1 1] Open/Close Chest
  (|CallParentFunction)
  (Variables|Default|SetRelative%20Rotation (Variables|/Script/Engine.SceneComponent|GetRelativeRotation (Variables|Default|GetScene)))
  (if (Variables|Default|GetOpen)
    (bind _newtrack_0 (Timeline|ToggleChest PlayFromStart)
      (:Update
        (Transformation|SetRelativeRotation (Variables|Default|GetScene) (Math|Rotator|Lerp(Rotator) (select (Variables|Default|GetOpen) (Variables|Default|GetRelative%20Rotation) "0, 0, 0") (select (Variables|Default|GetOpen) "0, 0,-45.000000" (Variables|Default|GetRelative%20Rotation)) _newtrack_0 true) false false)))
    (else
      (Timeline|ToggleChest ReverseFromEnd))))

(fn ConstructionScript
  (|CallParentFunction))

(fn RetrieveLootInfo
  (return ""))