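; Base lootable container that one character at a time opens, supplying inventory, outline and map-tracking data.
; Interact runs on the server, multicasts the inventory widget toggle by container type and flips Open, whose RepNotify drives animation and gamepad movement lock.
; Leaving the sphere closes it; other users see an in-use popup.
; A timer waits for the player, then binds to quest objective links so matching containers can report their location.
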(event OnComponentEndOverlap(Sphere)
  (params (OverlappedComponent :type Primitive%20Component%20Object%20Reference) (OtherActor :type Actor%20Object%20Reference) (OtherComp :type Primitive%20Component%20Object%20Reference) (OtherBodyIndex :type Integer))
  ;[1 1 1] Interact - Open Loot
  ;;[1 1 1] Close Chest on End Overlap
  (if (== OtherActor (Variables|Default|GetCharacter))
    (if (Variables|Default|GetOpen)
      (Networking|SwitchHasAuthority
        (:Authority
          ;;[1 1 1] Run On Server
          (CallFunction|MCInventory)
          ;;;[1 1 1] Handles Opening the Chest Via Notify
          (Variables|Default|SetOpen (not (Variables|Default|GetOpen))))
        (:Remote
          (CallFunction|SRCloseChest))))))

(event Custom|SR_Interact
  (params (Character :type Character%20Object%20Reference))
  ;[1 1 1] Interact - Open Loot
  ;;[1 1 1] Run On Server
  (CallFunction|Interact Character))

(event Custom|MC_Inventory
  ;[1 1 1] Interact - Open Loot
  ;;[1 1 1] Toggle Chest Widget
  (bind _playercontroller (Class|ICharacter|PassPlayerController(Message) (Variables|Default|GetCharacter)))
  (Variables|Default|SetPlayer%20Controller _playercontroller)
  (bind _interact (Class|IPlayerController|ExternalInventoryConditions(Message) (Variables|Default|GetPlayer%20Controller)))
  (if _interact
    (switch Utilities|FlowControl|Switch|SwitchonE_ChestType (Variables|SetupinGame|GetContainerType)
      (:NewEnumerator0
        ;;;[1 1 1] Chest No Sort Options
        (Class|IPlayerController|ToggleContainerInventory(Message) (Variables|Default|GetPlayer%20Controller) (Variables|Default|GetInventoryComponent)))
      (:NewEnumerator1
        ;;;[1 1 1] Chest With Sort Options
        (Class|IPlayerController|ToggleExternalInventory(Message) (Variables|Default|GetPlayer%20Controller) (Variables|Default|GetInventoryComponent) false)))))

(event Custom|SR_CloseChest
  ;[1 1 1] Interact - Open Loot
  ;;[1 1 1] Close Chest on End Overlap
  ;;[1 1 1] Run On Server
  (CallFunction|MCInventory)
  ;;;[1 1 1] Handles Opening the Chest Via Notify
  (Variables|Default|SetOpen (not (Variables|Default|GetOpen))))

(event Custom|PlayerValidCheck
  ;[1 1 1] Binds Dispatcher To Pass Location if Container of Objective
  (Utilities|IsValid (Game|GetPlayerCharacter 0)
    (:Is%20Valid
      (Utilities|Time|ClearandInvalidateTimerbyHandle (stale EventBeginPlay _returnvalue))
      (EventDispatchers|BindEventtoQuestObjectiveLink (Actor|GetComponentbyClass (Game|GetPlayerCharacter 0) "/Game/FlexibleCombatSystem/Blueprints/Components/QuestReceiverComponent.QuestReceiverComponent_C") (EventDispatchers|CreateEvent :!event IsQuestContainer)))))

(event EventServerCloseContainer
  (params (Character :type Character%20Object%20Reference))
  ;[1 1 1] Interact - Open Loot
  ;;[1 1 1] Run On Server
  (CallFunction|SRInteract Character))

(event EventToggleAnimation
  (bind _character (Variables|Default|GetCharacter))
  (bind _charactermovement (Variables|/Script/Engine.Character|GetCharacterMovement _character))
  ;[1 1 1] Interact - Open Loot
  ;;[1 1 1] Toggle Animation, Disable Input if using Gamepad
  (bind _gamepad (Class|IPlayerController|PassControlInput(Message) (Game|GetPlayerController 0)))
  (if _gamepad
    (if (not (Variables|Default|GetOpen))
      (Pawn|Components|CharacterMovement|SetMovementMode _charactermovement "MOVE_Walking" 0)
      (else
        (Pawn|Components|CharacterMovement|DisableMovement _charactermovement)))))

(event EventBeginPlay
  ;[1 1 1] Binds Dispatcher To Pass Location if Container of Objective
  (bind _returnvalue (Utilities|Time|SetTimerbyEvent (delegate Custom|PlayerValidCheck) 2.0 true)))

(event EventInteract
  (params (Character :type Character%20Object%20Reference))
  ;[1 1 1] Interact - Open Loot
  ;;[1 1 1] Run On Server
  (if (Variables|Default|GetOpen)
    (if (== (Variables|Default|GetCharacter) Character)
      (Networking|SwitchHasAuthority :!label _label
        (:Authority
          (if (Variables|Default|GetOpen)
            _
            (else
              (bind _output_get (Variables|Default|SetCharacter Character))
              (Actor|SetOwner _output_get)))
          (CallFunction|MCInventory)
          ;;;[1 1 1] Handles Opening the Chest Via Notify
          (Variables|Default|SetOpen (not (Variables|Default|GetOpen)))))
      (elif (Pawn|IsLocallyControlled Character)
        (bind _returnvalue (UserInterface|CreateWidget "/Game/FlexibleCombatSystem/Widgets/Combat/WB_PopupText.WB_PopupText_C" 0 "Loot in Use!"))
        (UserInterface|Viewport|AddtoViewport _returnvalue 0)))
    (else
      (goto _label))))

(fn ConstructionScript)

(fn OnRepOpen
  (Class|ILootInterface|ToggleAnimation(Message) self))

(fn IsQuestContainer
  (params (Quest%20Receiver :type Quest%20Receiver%20Component%20Object%20Reference) (Quest%20Info :type S%20Quest%20Info%20Structure))
  ;[1 1 1] IF Quest Item is Part of Quest Pass Data (Updated Location) over to Quest Log
  (bind (_array_element _array_index) (Utilities|Array|ForEachLoopwithBreak (Utilities|Struct|BreakS_QuestInfo Quest%20Info) :!label _label)
    (:LoopBody
      (if (.ObjectiveHasTracking? (Utilities|Struct|BreakS_QuestObjectiveInfo _array_element))
        (bind _returnvalue (Game|GetCurrentLevelName true))
        (if (Utilities|Enum|Equal(Enum) _returnvalue (.ObjectiveMapName (Utilities|Struct|BreakS_QuestObjectiveInfo _array_element)))
          (if (Utilities|Enum|Equal(Enum) (Variables|SetupinGame|GetContainerName) (.ContainerNameIFItemLootedfromEnemyorChest (Utilities|Struct|BreakS_QuestObjectiveInfo _array_element)))
            (bind _array_element_2 (Utilities|Array|ForEachLoopwithBreak (Variables|SetupinGame|GetContainerInventory))
              (:LoopBody
                (if (Utilities|Enum|Equal(Enum) (Utilities|Struct|BreakS_ItemData (CallFunction|GetItemData (Utilities|Struct|BreakS_ItemSetupData _array_element_2))) (.ObjectiveName (Utilities|Struct|BreakS_QuestObjectiveInfo _array_element)))
                  (Default|PassObjectiveUpdatedLocation Quest%20Receiver (Utilities|Struct|MakeS_QuestObjectiveInfo (.ObjectiveName (Utilities|Struct|BreakS_QuestObjectiveInfo _array_element)) (.ContainerNameIFItemLootedfromEnemyorChest (Utilities|Struct|BreakS_QuestObjectiveInfo _array_element)) (.ObjectiveType (Utilities|Struct|BreakS_QuestObjectiveInfo _array_element)) (.TotalObjectiveNumber (Utilities|Struct|BreakS_QuestObjectiveInfo _array_element)) (.ObjectiveHasTracking? (Utilities|Struct|BreakS_QuestObjectiveInfo _array_element)) (.ObjectiveMapName (Utilities|Struct|BreakS_QuestObjectiveInfo _array_element)) (Transformation|GetActorLocation) self) _array_index)
                  (goto _label Break))))))))))

(fn PassMapTrackingInfo
  (bind _trackinginfo (Variables|SetupInGame|GetTrackingInfo))
  (return (.trackingtype _trackinginfo) (.trackdistance _trackinginfo) (.objectivetexture _trackinginfo) (.objectivetexturesize _trackinginfo)))

(fn RetrieveInventoryInfo
  (return (Utilities|Select :Index (Variables|SetupinGame|GetContainerType) :NewEnumerator0 "NewEnumerator1" :NewEnumerator1 "NewEnumerator4") (Variables|SetupinGame|GetContainerName) (Variables|SetupinGame|GetContainerImage) (Variables|SetupinGame|GetContainerInventory) (Variables|SetupinGame|GetUseDataTable?) (Variables|SetupInGame|GetGuaranteedDTLoot) (Variables|SetupInGame|GetContainerDataTable) (Variables|SetupInGame|GetContainerSize)))

(fn RetrieveLootInfo
  (return ""))

(fn RetrieveOutlineInfo
  (return (Variables|SetupinGame|GetContainerName) (Variables|SetupinGame|GetContainerRarity) "NewEnumerator1" 0 (Variables|Default|GetItem) (Variables|Default|GetItem2) 0 false))