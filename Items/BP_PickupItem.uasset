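; Base pickup item actor that builds its static or skeletal mesh from data-table item info and goes into the player's inventory on interact.
; Pickups are saved by level, object name and location, so collected items destroy themselves on BeginPlay.
; Spawn&Use dispatches by item type to empty consume, use and weapon events for children, with RepNotifies syncing mesh and outline removal.
; Quest items bind to the player's quest receiver to report their location.
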(event Custom|WeaponOnUse
  ;[1 1 1] Use Item, Called From Inventory
  ;;[0.2431 0.696 1] Open For Children To Use
)

(event Custom|UseItemOnUse
  ;[1 1 1] Use Item, Called From Inventory
  ;;[0.2431 0.696 1] Open For Children To Use
)

(event Custom|ConsumeOnUse
  ;[1 1 1] Use Item, Called From Inventory
  ;;[0.2431 0.696 1] Open For Children To Use
)

(event Custom|PlayerValidCheck
  ;[1 1 1] Begin Play Setup
  (Utilities|IsValid (Game|GetPlayerCharacter 0)
    (:Is%20Valid
      (Utilities|Time|ClearandInvalidateTimerbyHandle (stale EventBeginPlay _returnvalue))
      (Quest|SetupQuestDispatch))))

(event EventBeginPlay
  ;[1 1 1] Begin Play Setup
  (CallFunction|DestroyUnusedMesh)
  (CallFunction|PickedUpCheck)
  (CallFunction|PlayerValidCheck)
  (bind _returnvalue (Utilities|Time|SetTimerbyEvent (delegate Custom|PlayerValidCheck) 0.5 true)))

(event EventSpawn&Use
  (params (CharacterRef :type Character%20Object%20Reference) (ItemInfo :type S%20Slot%20Info%20Structure))
  ;[1 1 1] Use Item, Called From Inventory
  (Variables|References|SetCharacterRef CharacterRef)
  (Variables|Status|SetItemInfo ItemInfo)
  ;;[1 1 1] Destroys Outline Comp
  (Variables|Default|SetPickedUp true)
  (CallFunction|SpawnSetup)
  (if (Utilities|Enum|Equal(Enum) (Utilities|Struct|BreakS_ItemData (CallFunction|GetItemData (Utilities|Struct|BreakS_SlotInfo (Variables|Status|GetItemInfo)))) "NewEnumerator14")
    (CallFunction|ConsumeonUse)
    (elif (Utilities|Enum|Equal(Enum) (Utilities|Struct|BreakS_ItemData (CallFunction|GetItemData (Utilities|Struct|BreakS_SlotInfo (Variables|Status|GetItemInfo)))) "NewEnumerator21")
      (CallFunction|UseItemonUse)
      (else
        (CallFunction|WeapononUse)))))

(event EventToggleCollision
  (params (Enabled :type Boolean))
  ;[1 1 1] For Projectile Blocking
  (Collision|SetCollisionEnabled (Variables|Default|GetItemStatic) (select Enabled "QueryAndPhysics" "NoCollision")))

(event EventInteract
  (params (Character :type Character%20Object%20Reference))
  (bind _iteminfo (Variables|Status|GetItemInfo))
  (bind (_datatableinfo _quantity _slotnumber _itemid) (Utilities|Struct|BreakS_SlotInfo _iteminfo))
  ;[1 1 1] On Character Interact, Add Item To Inventory
  (Variables|References|SetCharacterRef Character)
  (bind _slotsrequired (CallFunction|NumberOfSlotsUsed (Variables|Status|GetItemInfo)))
  (bind _success (Default|InventorySpaceRemaining (Actor|GetComponentbyClass (Variables|References|GetCharacterRef) "/Game/FlexibleCombatSystem/Blueprints/Components/InventoryComponent.InventoryComponent_C") _slotsrequired false))
  (if _success
    (Default|AddtoInventory (Actor|GetComponentbyClass (Variables|References|GetCharacterRef) "/Game/FlexibleCombatSystem/Blueprints/Components/InventoryComponent.InventoryComponent_C") (Utilities|Struct|MakeS_SlotInfo _datatableinfo (select (== _quantity 0) 1 _quantity) _slotnumber _itemid) false (Transformation|GetActorLocation) (Utilities|GetObjectName self))
    (Audio|PlaySoundatLocation (CallFunction|PassSoundFX "PickupItem") (Transformation|GetActorLocation) "0, 0, 0" 1.0 1.0 0.0 0 0 0 0)
    (CallFunction|PassItemforSave)
    (CallFunction|DestroySelf)))

(fn ConstructionScript
  (bind _itemskeletal (Variables|Default|GetItemSkeletal))
  (bind _datasetup (Variables|Default|GetDataSetup))
  (bind (_datatableinfo _quantity) (Utilities|Struct|BreakS_ItemSetupData _datasetup))
  (bind _relativelocation (Variables|/Script/Engine.SceneComponent|GetRelativeLocation _itemskeletal))
  (bind (_quantity_2 _randomizequantity _quantitymin _quantitymax) (Utilities|Struct|BreakS_QuantityOptions _quantity))
  (bind _returnvalue (Math|Random|RandomIntegerinRange _quantitymin _quantitymax))
  (bind _returnvalue_2 (select _randomizequantity _returnvalue _quantity_2))
  (bind _s_slotinfo (Utilities|Struct|MakeS_SlotInfo _datatableinfo _returnvalue_2))
  (bind _datatableinfo_2 (Utilities|Struct|BreakS_SlotInfo _s_slotinfo))
  (bind _slotdata (CallFunction|GetItemData _datatableinfo_2))
  (bind (_itemmesh _isspawneditem _resourcecollectiontooltype _isquestitem _weaponvfxinfo _equipmentinfo) (Utilities|Struct|BreakS_ItemData _slotdata))
  (bind (_bowarmorskeletalmesh _smz_offset) (Utilities|Struct|BreakS_EquipmentInfo _equipmentinfo))
  (Variables|Status|SetItemInfo _s_slotinfo)
  (Utilities|IsValid _itemmesh
    (:Is%20Valid
      (Components|StaticMesh|SetStaticMesh (Variables|Default|GetItemStatic) _itemmesh))
    (:Is%20Not%20Valid
      _))
  (Utilities|IsValid _bowarmorskeletalmesh
    (:Is%20Valid
      (Class|SkinnedMeshComponent|SetSkeletalMesh (Variables|Default|GetItemSkeletal) _bowarmorskeletalmesh true)
      (Rendering|SetVisibility (Variables|Default|GetItemStatic) false false))
    (:Is%20Not%20Valid
      _))
  (Transformation|SetRelativeLocation _itemskeletal (Math|Vector|MakeVector (- (.x _relativelocation) _smz_offset) (.y _relativelocation) (.z _relativelocation)) false false))

(fn PassItemforSave
  ;[1 1 1] We Use Display Name + Actor Location As Display Name Is Unique Per Placed Object. We combine it with Actor Location and Map name to ensure all names generated are Unique
  (bind _returnvalue (Game|GetCurrentLevelName true))
  (Class|IGameMode|SavePickedUpItems(Message) (Game|GetGameMode) (Utilities|String|Append _returnvalue (Utilities|GetObjectName self) (Utilities|String|ToString(Vector) (Transformation|GetActorLocation)))))

(fn DestroySelf
  (Default|RemoveActorTag (Variables|Default|GetOutlineComponent))
  (Class|IWeaponInterface|DestroySelf&Attachments(Message) self)
  (Actor|DestroyActor))

(fn SpawnSetup
  ;[1 1 1] Remove Tag Overlap
  (CallFunction|SetMeshDestroy)
  (Components|DestroyComponent (Variables|Default|GetCapsule))
  ;[1 1 1] Set Equipment Comp Ref
  (Variables|Default|SetEquipmentComponent (Actor|GetComponentbyClass (Variables|References|GetCharacterRef) "/Game/FlexibleCombatSystem/Blueprints/Components/EquipmentComponent.EquipmentComponent_C")))

(fn InitializeItem
  (bind _datasetup (Variables|Default|GetDataSetup))
  (bind (_datatableinfo _quantity) (Utilities|Struct|BreakS_ItemSetupData _datasetup))
  (bind (_quantity_2 _randomizequantity _quantitymin _quantitymax) (Utilities|Struct|BreakS_QuantityOptions _quantity))
  (Variables|Status|SetItemInfo (Utilities|Struct|MakeS_SlotInfo _datatableinfo (select _randomizequantity (Math|Random|RandomIntegerinRange _quantitymin _quantitymax) _quantity_2))))

(fn SetMesh
  (bind _itemstatic (Variables|Default|GetItemStatic))
  (bind _itemskeletal (Variables|Default|GetItemSkeletal))
  (bind _iteminfo (Variables|Status|GetItemInfo))
  (bind _datatableinfo (Utilities|Struct|BreakS_SlotInfo _iteminfo))
  (bind _slotdata (CallFunction|GetItemData _datatableinfo))
  (bind (_itemmesh _isspawneditem _resourcecollectiontooltype _isquestitem _weaponvfxinfo _equipmentinfo) (Utilities|Struct|BreakS_ItemData _slotdata))
  (bind _bowarmorskeletalmesh (Utilities|Struct|BreakS_EquipmentInfo _equipmentinfo))
  ;[1 1 1] Set Meshes, Destroy the One Not Used
  (Utilities|IsValid _itemmesh
    (:Is%20Valid
      (Components|StaticMesh|SetStaticMesh _itemstatic _itemmesh)
      (Rendering|SetVisibility _itemstatic true false)
      (Variables|Default|SetUpdateMeshNotify false))
    (:Is%20Not%20Valid
      (Variables|Default|SetUpdateMeshNotify true)))
  (Utilities|IsValid _bowarmorskeletalmesh
    (:Is%20Valid
      (Class|SkinnedMeshComponent|SetSkeletalMesh _itemskeletal _bowarmorskeletalmesh true)
      (Rendering|SetVisibility _itemskeletal true false))))

(fn SetMeshDestroy
  ;[1 1 1] Set Meshes, Destroy the One Not Used
  ;;[1 1 1] Replicates "Set Mesh" To Clients
  (Variables|Default|SetUpdateMeshNotify true)
  (Utilities|IsValid (Utilities|Struct|BreakS_ItemData (CallFunction|GetItemData (Utilities|Struct|BreakS_SlotInfo (Variables|Status|GetItemInfo))))
    (:Is%20Valid
      (Variables|Default|SetStaticORSkeletal false))
    (:Is%20Not%20Valid
      (Variables|Default|SetStaticORSkeletal true))))

(fn PickedUpCheck
  ;[1 1 1] Checks IF Picked Up - Destroys IF Is
  (bind _returnvalue (SaveGame|LoadGamefromSlot (CallFunction|RetreiveSaveSlotName)))
  (bind _asbp_save_game (Utilities|Casting|CastToBP_SaveGame _returnvalue))
  (bind _returnvalue_2 (Game|GetCurrentLevelName true))
  (bind _array_element (Utilities|Array|ForEachLoopwithBreak (Variables|/Game/FlexibleCombatSystem/Blueprints/BP_SaveGame.BP_SaveGame_C|GetPickedUpActors _asbp_save_game) :!label _label)
    (:LoopBody
      (if (Utilities|Enum|Equal(Enum) _array_element (Utilities|String|Append _returnvalue_2 (Utilities|GetObjectName self) (Utilities|String|ToString(Vector) (Transformation|GetActorLocation))))
        (Actor|DestroyActor)
        (goto _label Break)))))

(fn OnRepPickedUp
  (bind _outlinecomponent (Variables|Default|GetOutlineComponent))
  ;[1 1 1] Replicates To Clients - Prevents Outline Component Triggering After Pickup
  (Default|RemoveActorTag _outlinecomponent)
  (Components|DestroyComponent _outlinecomponent))

(fn PassQuestObjectiveData
  (params (Quest%20Receiver :type Quest%20Receiver%20Component%20Object%20Reference) (Quest%20Info :type S%20Quest%20Info%20Structure))
  ;[1 1 1] IF Quest Item is Part of Quest Pass Data (Updated Location) over to Quest Log
  (bind (_array_element _array_index) (Utilities|Array|ForEachLoopwithBreak (Utilities|Struct|BreakS_QuestInfo Quest%20Info) :!label _label)
    (:LoopBody
      (if (Utilities|Enum|Equal(Enum) (Utilities|Struct|BreakS_ItemData (CallFunction|GetItemData (Utilities|Struct|BreakS_SlotInfo (Variables|Status|GetItemInfo)))) (.ObjectiveName (Utilities|Struct|BreakS_QuestObjectiveInfo _array_element)))
        (if (.ObjectiveHasTracking? (Utilities|Struct|BreakS_QuestObjectiveInfo _array_element))
          (bind _returnvalue (Game|GetCurrentLevelName true))
          (if (Utilities|Enum|Equal(Enum) _returnvalue (.ObjectiveMapName (Utilities|Struct|BreakS_QuestObjectiveInfo _array_element)))
            (Default|PassObjectiveUpdatedLocation Quest%20Receiver (Utilities|Struct|MakeS_QuestObjectiveInfo (.ObjectiveName (Utilities|Struct|BreakS_QuestObjectiveInfo _array_element)) "" (.ObjectiveType (Utilities|Struct|BreakS_QuestObjectiveInfo _array_element)) (.TotalObjectiveNumber (Utilities|Struct|BreakS_QuestObjectiveInfo _array_element)) (.ObjectiveHasTracking? (Utilities|Struct|BreakS_QuestObjectiveInfo _array_element)) (.ObjectiveMapName (Utilities|Struct|BreakS_QuestObjectiveInfo _array_element)) (Transformation|GetActorLocation) self) _array_index)
            (goto _label Break)))))))

(fn SetupQuestDispatch
  ;[1 1 1] Binds Quest Objective to Event Dispatcher - End Result to Pass Location over to Quest Log
  (if (Utilities|Struct|BreakS_ItemData (CallFunction|GetItemData (Utilities|Struct|BreakS_SlotInfo (Variables|Status|GetItemInfo))))
    (EventDispatchers|BindEventtoQuestObjectiveLink (Actor|GetComponentbyClass (Game|GetPlayerCharacter 0) "/Game/FlexibleCombatSystem/Blueprints/Components/QuestReceiverComponent.QuestReceiverComponent_C") (EventDispatchers|CreateEvent :!event PassQuestObjectiveData))))

(fn OnRepUpdateMeshNotify
  (bind _iteminfo (Variables|Status|GetItemInfo))
  (bind _itemskeletal (Variables|Default|GetItemSkeletal))
  (bind _itemstatic (Variables|Default|GetItemStatic))
  (bind _datatableinfo (Utilities|Struct|BreakS_SlotInfo _iteminfo))
  (bind _slotdata (CallFunction|GetItemData _datatableinfo))
  (bind (_itemmesh _equipmentinfo) (Utilities|Struct|BreakS_ItemData _slotdata))
  (bind _bowarmorskeletalmesh (Utilities|Struct|BreakS_EquipmentInfo _equipmentinfo))
  ;[1 1 1] Set Mesh
  (Utilities|IsValid _itemmesh
    (:Is%20Valid
      (Components|StaticMesh|SetStaticMesh _itemstatic _itemmesh)
      (Rendering|SetVisibility _itemstatic true false))
    (:Is%20Not%20Valid
      (bind _itemstatic_2 (Variables|Default|GetItemStatic)
        (:then
          (Components|DestroyComponent _itemstatic_2))
        (:else
          _))))
  (Utilities|IsValid _bowarmorskeletalmesh
    (:Is%20Valid
      (Class|SkinnedMeshComponent|SetSkeletalMesh _itemskeletal _bowarmorskeletalmesh true)
      (Rendering|SetVisibility _itemskeletal true false))
    (:Is%20Not%20Valid
      (bind _itemskeletal_2 (Variables|Default|GetItemSkeletal)
        (:then
          (Components|DestroyComponent _itemskeletal_2))
        (:else)))))

(fn DestroyUnusedMesh
  (bind _itemskeletal (Variables|Default|GetItemSkeletal))
  (bind _datasetup (Variables|Default|GetDataSetup))
  (bind _itemstatic (Variables|Default|GetItemStatic))
  (bind _datatableinfo (Utilities|Struct|BreakS_ItemSetupData _datasetup))
  (bind _s_slotinfo (Utilities|Struct|MakeS_SlotInfo _datatableinfo))
  (bind _datatableinfo_2 (Utilities|Struct|BreakS_SlotInfo _s_slotinfo))
  (bind _slotdata (CallFunction|GetItemData _datatableinfo_2))
  (bind (_itemmesh _equipmentinfo) (Utilities|Struct|BreakS_ItemData _slotdata))
  (bind _bowarmorskeletalmesh (Utilities|Struct|BreakS_EquipmentInfo _equipmentinfo))
  (if (or (Utilities|IsValid _itemmesh) (Utilities|IsValid (Utilities|Struct|BreakS_EquipmentInfo _equipmentinfo)))
    (Utilities|IsValid _itemmesh
      (:Is%20Valid
        (Components|StaticMesh|SetStaticMesh _itemstatic _itemmesh))
      (:Is%20Not%20Valid
        (Utilities|IsValid _itemstatic
          (:Is%20Valid
            (Components|DestroyComponent _itemstatic))
          (:Is%20Not%20Valid
            _))))
    (Utilities|IsValid _bowarmorskeletalmesh
      (:Is%20Valid
        (Class|SkinnedMeshComponent|SetSkeletalMesh _itemskeletal _bowarmorskeletalmesh true))
      (:Is%20Not%20Valid
        (Utilities|IsValid _itemskeletal
          (:Is%20Valid
            (Components|DestroyComponent _itemskeletal)))))))

(fn RetrieveOutlineInfo
  (bind _itemstatic (Variables|Default|GetItemStatic))
  (bind _itemskeletal (Variables|Default|GetItemSkeletal))
  (bind _iteminfo (Variables|Status|GetItemInfo))
  (bind (_datatableinfo _quantity) (Utilities|Struct|BreakS_SlotInfo _iteminfo))
  (bind _slotdata (CallFunction|GetItemData _datatableinfo))
  (bind (_name _itemrarity) (Utilities|Struct|BreakS_ItemData _slotdata))
  (return _name _itemrarity "NewEnumerator0" _quantity (select (Utilities|IsValid _itemstatic) _itemstatic 0) 0 (select (Utilities|IsValid _itemskeletal) _itemskeletal 0) false))