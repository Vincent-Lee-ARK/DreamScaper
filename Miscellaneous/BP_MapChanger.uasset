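; BP_MapChanger is a trigger volume that switches the minimap and world map when the local player enters it.
; A box overlap checks for a locally controlled, Player-tagged character, and a looping startup timer catches a player already inside once the pawn is valid.
; The update looks up its row in DT_MapData, then passes the map info to the HUD minimap widget and player controller.
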(event OnComponentBeginOverlap(Box)
  (params (OverlappedComponent :type Primitive%20Component%20Object%20Reference) (OtherActor :type Actor%20Object%20Reference) (OtherComp :type Primitive%20Component%20Object%20Reference) (OtherBodyIndex :type Integer) (bFromSweep :type Boolean) (SweepResult :type Hit%20Result%20Structure%20%28by%20ref%29))
  ;[1 1 1] Location Trigger
  (bind _ascharacter (Utilities|Casting|CastToCharacter OtherActor))
  (if (Pawn|IsLocallyControlled _ascharacter)
    (if (Actor|ActorHasTag OtherActor "Player")
      (CallFunction|UpdateMap))))

(event Custom|UpdateMap
  ;[1 1 1] Update Map
  (bind _hudref (Class|IPlayerController|PassHUDWB(Message) (Game|GetPlayerController 0)))
  (bind _returnvalue (Utilities|GetDataTableRow "/Game/FlexibleCombatSystem/DataTables/DT_MapData.DT_MapData" (Variables|Default|GetMapName%20%28MapData%20DT%29))
    (:then
      (Default|UpdateMap (Variables|/Game/FlexibleCombatSystem/Widgets/HUD/WB_HUD.WB_HUD_C|GetWB_MiniMap _hudref) (.MiniMapInfo (Utilities|Struct|BreakS_MapTextureInfo _returnvalue)))
      (Class|IPlayerController|ToggleSpecificMap(Message) (Game|GetPlayerController 0) (.WorldMapInfo (Utilities|Struct|BreakS_MapTextureInfo _returnvalue))))))

(event Custom|PlayerValidCheck
  ;[1 1 1] Bind Quest Objective Link
  (Utilities|IsValid (Game|GetPlayerCharacter 0)
    (:Is%20Valid
      (if (Collision|IsOverlappingActor (Game|GetPlayerCharacter 0) self :!class /Script/Engine.Actor)
        (CallFunction|UpdateMap))
      (Utilities|Time|ClearandInvalidateTimerbyHandle (stale EventBeginPlay _returnvalue)))))

(event EventBeginPlay
  ;[1 1 1] Bind Quest Objective Link
  (bind _returnvalue (Utilities|Time|SetTimerbyEvent (delegate Custom|PlayerValidCheck) 0.2 true)))

(fn ConstructionScript)