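; Activate Actor child for actors the player activates by interacting, adding an Outline Component on top of the parent logic.
; On BeginPlay it destroys the outline if activation was saved, or deactivates it for quest actors until the parent's quest dispatcher makes them activateable.
; Interaction disables further activation and clears the outline's active state and actor tag.
; RetrieveOutlineInfo supplies the name, tag type and meshes for the outline.
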(event EventBeginPlay
  ;[1 1 1] Child of Activate Actor Parent, this BP adds in the Outline Component for Actors that are going to be activated by the player interacting with them
  (|CallParentFunction)
  (if (Variables|Default|GetSaveActivated)
    (Components|DestroyComponent (Variables|Default|GetOutlineComponent))
    (elif (Variables|Default|GetIsQuestActor)
      (Variables|/Game/FlexibleCombatSystem/Blueprints/Components/OutlineComponent.OutlineComponent_C|SetActorIsActive (Variables|Default|GetOutlineComponent) false))))

(event EventSetActortoActivateable
  ;[1 1 1] Child of Activate Actor Parent, this BP adds in the Outline Component for Actors that are going to be activated by the player interacting with them
  ;;[1 1 1] Called when Quest is Linked through Event Dispatcher - See Parent
  (|CallParentFunction)
  (bind _outlinecomponent (Variables|Default|GetOutlineComponent)
    (:then
      (Variables|/Game/FlexibleCombatSystem/Blueprints/Components/OutlineComponent.OutlineComponent_C|SetActorIsActive _outlinecomponent true))
    (:else)))

(event EventMCInteract
  (bind _outlinecomponent (Variables|Default|GetOutlineComponent))
  ;[1 1 1] Child of Activate Actor Parent, this BP adds in the Outline Component for Actors that are going to be activated by the player interacting with them
  (|CallParentFunction)
  (Variables|Default|SetCanBeActivated false)
  (Variables|/Game/FlexibleCombatSystem/Blueprints/Components/OutlineComponent.OutlineComponent_C|SetActorIsActive _outlinecomponent false)
  (Default|RemoveActorTag _outlinecomponent))

(fn ConstructionScript
  (|CallParentFunction))

(fn RetrieveOutlineInfo
  (return (Variables|Default|GetActivateActorName) "NewEnumerator0" "NewEnumerator7" 0 (Variables|Default|GetMesh%201) (Variables|Default|GetMesh%202) 0 false))