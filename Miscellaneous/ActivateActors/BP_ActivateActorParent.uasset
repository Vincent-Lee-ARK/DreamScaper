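; Parent Blueprint for interactable actors that activate, persist in the save game and can serve as quest objectives.
; BeginPlay instantly reactivates saved actors and polls until the player's QuestReceiverComponent exists, then binds quest events.
; Interact, gated by CanBeActivated, reports quest progress locally, saves through the GameMode and multicasts on authority.
; Quest helpers unlock matching actors and pass tracked locations, while activation events are empty hooks.
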(event Custom|InstantActivate
  ;[1 1 1] Activates Actor If In Save
  ;;[1 1 1] Save Game Activate
  ;;;[1 1 1] Activates the Actor Instantly
)

(event Custom|SetActorToActivateable
  ;[1 1 1] Activates Actor If In Save
  ;;[0.7208 0.7072 1] Used For Quest Activation Actors which we dont want to enable straight away. Gets updated when Quest is Accepted
  (Variables|Default|SetCanBeActivated true))

(event Custom|SR_Interact
  ;[1 1 1] Activates Actor If In Save
  ;;[0.2812 0.6512 1] RPCs
  (CallFunction|MCInteract))

(event Custom|PlayerValidCheck
  ;[1 1 1] Activates Actor If In Save
  (Utilities|IsValid (Actor|GetComponentbyClass (Game|GetPlayerCharacter 0) "/Game/FlexibleCombatSystem/Blueprints/Components/QuestReceiverComponent.QuestReceiverComponent_C")
    (:Is%20Valid
      (Utilities|Time|ClearandInvalidateTimerbyHandle (stale EventBeginPlay _returnvalue))
      (CallFunction|SetupObjectiveLink))))

(event Custom|MC_Interact
  ;[1 1 1] Activates Actor If In Save
  ;;[0.2812 0.6512 1] RPCs
)

(event EventBeginPlay
  ;[1 1 1] Activates Actor If In Save
  (bind _returnvalue (Utilities|Time|SetTimerbyEvent (delegate Custom|PlayerValidCheck) 2.0 true))
  ;;[1 1 1] Save Game Activate
  (bind _returnvalue_2 (SaveGame|LoadGamefromSlot (CallFunction|RetreiveSaveSlotName)))
  (bind _asbp_save_game (Utilities|Casting|CastToBP_SaveGame _returnvalue_2))
  (bind _array_element (Utilities|Array|ForEachLoopwithBreak (Variables|/Game/FlexibleCombatSystem/Blueprints/BP_SaveGame.BP_SaveGame_C|GetActivatedActors _asbp_save_game) :!label _label)
    (:LoopBody
      (bind _returnvalue_3 (Game|GetCurrentLevelName true))
      (if (and (Utilities|Enum|Equal(Enum) _returnvalue_3 (.MapName (Utilities|Struct|BreakS_ActorSaveInfo _array_element))) (Utilities|Enum|Equal(Enum) (.ActorName (Utilities|Struct|BreakS_ActorSaveInfo _array_element)) (Utilities|GetObjectName self)))
        (CallFunction|InstantActivate)
        (Variables|Default|SetSaveActivated true)
        (goto _label Break)))))

(event EventInteract
  (params (Character :type Character%20Object%20Reference))
  ;[1 1 1] Activates Actor If In Save
  ;;[1 1 1] Activate
  (if (Variables|Default|GetCanBeActivated)
    (Utilities|IsValid Character
      (:Is%20Valid
        (if (Pawn|IsLocallyControlled Character)
          (CallFunction|IsQuestActor (Game|GetPlayerCharacter 0) (Variables|Default|GetActivateActorName) 1 (Transformation|GetActorLocation) (Utilities|GetObjectName self))))
      (:Is%20Not%20Valid
        _))
    ;;[1 1 1] Save Activation
    (Class|IGameMode|SaveActorActivated(Message) (Game|GetGameMode) (Utilities|GetObjectName self))
    ;;[0.2812 0.6512 1] RPCs
    (Networking|SwitchHasAuthority
      (:Authority
        (CallFunction|MCInteract)))))

(fn ConstructionScript)

(fn SetupObjectiveLink
  (bind _returnvalue (Game|GetPlayerCharacter 0))
  (bind _returnvalue_2 (Actor|GetComponentbyClass _returnvalue "/Game/FlexibleCombatSystem/Blueprints/Components/QuestReceiverComponent.QuestReceiverComponent_C"))
  ;[1 1 1] Binds Dispatcher To Pass Location if Interact Quest Objective
  (if (Variables|Default|GetIsQuestActor)
    (EventDispatchers|BindEventtoQuestObjectiveLink _returnvalue_2 (EventDispatchers|CreateEvent :!event PassQuestObjectiveData))
    (EventDispatchers|BindEventtoQuestAccepted _returnvalue_2 (EventDispatchers|CreateEvent :!event IsQuestObjectiveCheck))))

(fn PassQuestObjectiveData
  (params (Quest%20Receiver :type Quest%20Receiver%20Component%20Object%20Reference) (Quest%20Info :type S%20Quest%20Info%20Structure))
  ;[1 1 1] IF Quest Item is Part of Quest Pass Data (Updated Location) over to Quest Log
  (bind (_array_element _array_index) (Utilities|Array|ForEachLoopwithBreak (.QuestObjectiveInfo (Utilities|Struct|BreakS_QuestInfo Quest%20Info)) :!label _label)
    (:LoopBody
      (if (Utilities|Enum|Equal(Enum) (Variables|Default|GetActivateActorName) (.ObjectiveName (Utilities|Struct|BreakS_QuestObjectiveInfo _array_element)))
        (if (.ObjectiveHasTracking? (Utilities|Struct|BreakS_QuestObjectiveInfo _array_element))
          (bind _returnvalue (Game|GetCurrentLevelName true))
          (if (Utilities|Enum|Equal(Enum) _returnvalue (.ObjectiveMapName (Utilities|Struct|BreakS_QuestObjectiveInfo _array_element)))
            (Default|PassObjectiveUpdatedLocation Quest%20Receiver (Utilities|Struct|MakeS_QuestObjectiveInfo (.ObjectiveName (Utilities|Struct|BreakS_QuestObjectiveInfo _array_element)) "" (.ObjectiveType (Utilities|Struct|BreakS_QuestObjectiveInfo _array_element)) (.TotalObjectiveNumber (Utilities|Struct|BreakS_QuestObjectiveInfo _array_element)) (.ObjectiveHasTracking? (Utilities|Struct|BreakS_QuestObjectiveInfo _array_element)) (.ObjectiveMapName (Utilities|Struct|BreakS_QuestObjectiveInfo _array_element)) (Transformation|GetActorLocation) self) _array_index)
            (goto _label Break)))))))

(fn IsQuestObjectiveCheck
  (params (QuestInfo :type S%20Quest%20Storage%20Info%20Structure) (LoadingSaveData :type Boolean))
  (for _array_element (Utilities|Struct|BreakS_QuestStorageInfo QuestInfo)
    (if (Utilities|Enum|Equal(Enum) (.ObjectiveName (Utilities|Struct|BreakS_QuestObjectiveStatus _array_element)) (Variables|Default|GetActivateActorName))
      (CallFunction|SetActortoActivateable)
      (return))))