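; Placeable quest trigger volume that auto-accepts a quest when the player walks into it.
; A looping timer polls for a valid player character, then initializes the QuestGiverComponent with QuestsToOffer.
; Box overlap by a locally controlled, Player-tagged character opens the next unaccepted quest through that component, passing along ActorToActivate.
; PassMapTrackingInfo exposes the TrackingInfo fields for map tracking.
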(event OnComponentBeginOverlap(Box)
  (params (OverlappedComponent :type Primitive%20Component%20Object%20Reference) (OtherActor :type Actor%20Object%20Reference) (OtherComp :type Primitive%20Component%20Object%20Reference) (OtherBodyIndex :type Integer) (bFromSweep :type Boolean) (SweepResult :type Hit%20Result%20Structure%20%28by%20ref%29))
  (bind _questgivercomponent (Variables|Default|GetQuestGiverComponent))
  ;[1 1 1] Location Trigger
  (bind _ascharacter (Utilities|Casting|CastToCharacter OtherActor))
  (if (Pawn|IsLocallyControlled _ascharacter)
    (if (Actor|ActorHasTag OtherActor "Player")
      (if (not (Variables|/Game/FlexibleCombatSystem/Blueprints/Components/QuestGiverComponent.QuestGiverComponent_C|GetQuestAccepted _questgivercomponent))
        (if (not (> (Variables|/Game/FlexibleCombatSystem/Blueprints/Components/QuestGiverComponent.QuestGiverComponent_C|GetQuestNumber _questgivercomponent) (Variables|/Game/FlexibleCombatSystem/Blueprints/Components/QuestGiverComponent.QuestGiverComponent_C|GetNumberOfQuests _questgivercomponent)))
          (Default|OpenQuest (Variables|Default|GetQuestGiverComponent) (Variables|SetupInGame|GetActor%20to%20Activate) true))))))

(event Custom|PlayerValidCheck
  ;[1 1 1] Bind Quest Objective Link
  (Utilities|IsValid (Game|GetPlayerCharacter 0)
    (:Is%20Valid
      (Utilities|Time|ClearandInvalidateTimerbyHandle (stale EventBeginPlay _returnvalue))
      (if (> (Utilities|Array|Length (Variables|SetupInGame|GetQuestsToOffer)) 0)
        (Default|InitializeQuestGiver (Variables|Default|GetQuestGiverComponent) 0 (Variables|SetupInGame|GetQuestsToOffer))))))

(event EventBeginPlay
  ;[1 1 1] Bind Quest Objective Link
  (CallFunction|PlayerValidCheck)
  (bind _returnvalue (Utilities|Time|SetTimerbyEvent (delegate Custom|PlayerValidCheck) 0.5 true)))

(fn ConstructionScript)

(fn PassMapTrackingInfo
  (bind _trackinginfo (Variables|SetupInGame|GetTrackingInfo))
  (return (.trackingtype _trackinginfo) (.trackdistance _trackinginfo) (.objectivetexture _trackinginfo) (.objectivetexturesize _trackinginfo)))